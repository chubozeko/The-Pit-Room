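; BP_Tracker is a calibration actor representing a motion capture tracker attached to a skeleton bone, labeled with its name.
; Capture pawn hands register it on overlap with a highlight.
; In keyboard mode, clicking registers it with the spectator pawn and spawns a translation or rotation manipulator with local/world space toggling.
; Reattachment optionally changes the bone, keeps world transform, then sends the inverted relative transform to the capture device as offset.
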(event OnComponentBeginOverlap(StaticMesh)
  (params (OverlappedComponent :type Primitive%20Component%20Object%20Reference) (OtherActor :type Actor%20Object%20Reference) (OtherComp :type Primitive%20Component%20Object%20Reference) (OtherBodyIndex :type Integer) (bFromSweep :type Boolean) (SweepResult :type Hit%20Result%20Structure%20%28by%20ref%29))
  (bind _self self)
  ;[1 1 1] Enable Highlighting on overlap
  (bind _player (Utilities|OverlappingPlayerHand OtherActor OtherComp)
    (:IsPlayer
      (if (Components|ComponentHasTag OtherComp "RIGHT")
        (Variables|/Game/VMK/Blueprints/BP_CapturePawn.BP_CapturePawn_C|SetRightHandTracker _player _self)
        (else
          (Variables|/Game/VMK/Blueprints/BP_CapturePawn.BP_CapturePawn_C|SetLeftHandTracker _player _self)))
      (Rendering|SetRenderCustomDepth (Variables|Default|GetStaticMesh) true))))

(event OnComponentEndOverlap(StaticMesh)
  (params (OverlappedComponent :type Primitive%20Component%20Object%20Reference) (OtherActor :type Actor%20Object%20Reference) (OtherComp :type Primitive%20Component%20Object%20Reference) (OtherBodyIndex :type Integer))
  ;[1 1 1] Enable Highlighting on overlap
  (bind _player (Utilities|OverlappingPlayerHand OtherActor OtherComp)
    (:IsPlayer
      (if (Components|ComponentHasTag OtherComp "RIGHT")
        (Variables|/Game/VMK/Blueprints/BP_CapturePawn.BP_CapturePawn_C|SetRightHandTracker _player 0)
        (else
          (Variables|/Game/VMK/Blueprints/BP_CapturePawn.BP_CapturePawn_C|SetLeftHandTracker _player 0)))
      (Rendering|SetRenderCustomDepth (Variables|Default|GetStaticMesh) false))))

(event OnBeginCursorOver(StaticMesh)
  (params (TouchedComponent :type Primitive%20Component%20Object%20Reference))
  ;[1 1 1] Keyboard: Select object
  (if (Variables|Settings|GetKeyboardControl)
    (Rendering|SetRenderCustomDepth (Variables|Default|GetStaticMesh) true)))

(event OnEndCursorOver(StaticMesh)
  (params (TouchedComponent :type Primitive%20Component%20Object%20Reference))
  ;[1 1 1] Keyboard: Select object
  (if (Variables|Settings|GetKeyboardControl)
    (if (not (Variables|Settings|GetKeyboardSelected))
      (Rendering|SetRenderCustomDepth (Variables|Default|GetStaticMesh) false))))

(event OnClicked(StaticMesh)
  (params (TouchedComponent :type Primitive%20Component%20Object%20Reference) (ButtonPressed :type Key%20Structure :default "None"))
  ;[1 1 1] Keyboard: Select object
  (if (Variables|Settings|GetKeyboardControl)
    (if (not (Variables|Settings|GetKeyboardSelected))
      (Variables|Settings|SetKeyboardSelected true)
      (CallFunction|SpawnManipulator "/Game/VMK/Blueprints/Manipulators/BP_ToolTranslation.BP_ToolTranslation_C")
      (Variables|Settings|SetKeyboardUseRotation false)
      ;[1 1 1] Update Reference
      (bind _asbp_player_spectator_2d (Utilities|Casting|CastToBP_PlayerSpectator2D (Game|Player|GetPlayerPawn 0)))
      (Default|SetActiveTracker _asbp_player_spectator_2d self)
      (Variables|Default|SetNewBoneName (Variables|Default|GetBone)))))

(event Custom|UpdateLabel
  (bind _tags (Variables|Actor|GetTags))
  (bind _output (Utilities|Array|Get(acopy) _tags))
  (bind _returnvalue (Utilities|Text|ToText(Name) _output))
  ;[1 1 1] Basic Setup
  (if (Utilities|Array|IsValidIndex _tags)
    (if (Utilities|Enum|NotEqual(Enum) _returnvalue (Variables|/Script/Engine.TextRenderComponent|GetText (Variables|Default|GetTX_Bone)))
      (Rendering|Components|TextRender|SetText (Variables|Default|GetTX_Bone) _returnvalue))))

(event Custom|ToggleManipulatorSpace
  (Utilities|IsValid (Variables|Default|GetCurrentManipulator)
    (:Is%20Valid
      (Variables|Default|SetbManipulatorLocalSpace (not (Variables|Default|GetbManipulatorLocalSpace)))
      (CallFunction|UpdateManipulatorSpace))))

(event Custom|StopControl
  (bind _currentmanipulator (Variables|Default|GetCurrentManipulator))
  ;[1 1 1] Actions on Deactivate: destroy manipulator, mark as unselected
  (Utilities|IsValid _currentmanipulator
    (:Is%20Valid
      (Actor|DestroyActor _currentmanipulator))
    (:Is%20Not%20Valid
      _))
  (Variables|Settings|SetKeyboardSelected false)
  (Rendering|SetRenderCustomDepth (Variables|Default|GetStaticMesh) false))

(event Custom|UpdateCalibration
  ;[1 1 1] Update Tracker's offset
  (if (Variables|Settings|GetKeyboardControl)
    (CallFunction|RestoreAttachment (Variables|Default|GetCapDevice) true)
    (|ResetManipulatortoWorldSpace)))

(event Custom|SpawnManipulator
  (params (Class :type Static%20Mesh%20Actor%20Object%20Reference))
  ;[1 1 1] Spawn Tool for Rotation/Location
  (Utilities|IsValid (Variables|Default|GetCurrentManipulator)
    (:Is%20Valid
      (Actor|DestroyActor (Variables|Default|GetCurrentManipulator)))
    (:Is%20Not%20Valid
      _))
  (bind _returnvalue (Game|SpawnActorfromClass Class (Math|Transform|MakeTransform "0, 0, 0") "AlwaysSpawn" 0 0))
  (bind _output_get (Variables|Default|SetCurrentManipulator _returnvalue))
  (Transformation|AttachComponentToComponent _output_get (Variables|Debug|GetStaticMeshComponent) "None" "SnapToTarget" "SnapToTarget" "SnapToTarget" true)
  (CallFunction|UpdateManipulatorSpace))

(event Custom|InitForCalibration
  (params (TrackerName :type Text) (TrackerId :type Byte) (Bone :type Name) (Owner :type BP%20Manual%20Calibration%20Object%20Reference))
  (bind _staticmesh (Variables|Default|GetStaticMesh))
  ;[1 1 1] Attach Tracker to player's hand
  (Variables|Default|SetIndex TrackerId)
  (Variables|Default|SetBone Bone)
  (Variables|Default|SetOwnerCalibrator Owner)
  (Collision|SetCollisionEnabled (Variables|Default|GetStaticMesh) "QueryOnly")
  (Utilities|Time|ClearTimerbyFunctionName 0 "UpdateLabel")
  (Rendering|Components|TextRender|SetText (Variables|Default|GetTX_Bone) TrackerName)
  (Rendering|SetVisibility (Variables|Default|GetTX_Bone) true false)
  (if (and (Utilities|Array|ContainsItem (Class|SteamVRFunctionLibrary|GetValidTrackedDeviceIds "Controller") (Math|Conversions|ToInteger(Byte) (Variables|Default|GetIndex))) (not (Variables|Settings|GetKeyboardControl)))
    (Transformation|SetRelativeLocationAndRotation _staticmesh "0, 0, 0" "0, 0, 0" false false)
    (Components|StaticMesh|SetStaticMesh _staticmesh "/Engine/VREditor/Devices/Vive/VivePreControllerMesh.VivePreControllerMesh")))

(event Custom|ToggleManipulationMode
  (params (IsRotation :type Boolean))
  ;[1 1 1] Toggle Move/Rotate Mode
  (bind _output_get (Variables|Settings|SetKeyboardUseRotation IsRotation))
  (CallFunction|SpawnManipulator (select _output_get "/Game/VMK/Blueprints/Manipulators/BP_ToolRotation.BP_ToolRotation_C" "/Game/VMK/Blueprints/Manipulators/BP_ToolTranslation.BP_ToolTranslation_C")))

(event Custom|UpdateManipulatorSpace
  (bind _currentmanipulator (Variables|Default|GetCurrentManipulator))
  (bind _currentmanipulator_2 (Variables|Default|GetCurrentManipulator))
  (bind _rootcomponent (Variables|/Script/Engine.Actor|GetRootComponent _currentmanipulator))
  (if (Variables|Default|GetbManipulatorLocalSpace)
    (Transformation|SetRelativeRotation _rootcomponent "0, 0, 0" false false)
    (bind _asbp_tool_rotation (Utilities|Casting|CastToBP_ToolRotation _currentmanipulator_2))
    (Variables|/Game/VMK/Blueprints/Manipulators/BP_ToolRotation.BP_ToolRotation_C|SetbIsLocal _asbp_tool_rotation true)
    (else
      (Transformation|SetWorldRotation _rootcomponent "0, 0, 0" false false)
      (bind _asbp_tool_rotation_2 (Utilities|Casting|CastToBP_ToolRotation _currentmanipulator_2))
      (Variables|/Game/VMK/Blueprints/Manipulators/BP_ToolRotation.BP_ToolRotation_C|SetbIsLocal _asbp_tool_rotation_2 false))))

(event Custom|RestoreAttachment
  (params (CapDevice :type Capture%20Device%20Object%20Reference) (CanUpdateBone :type Boolean))
  (bind _ownercalibrator (Variables|Default|GetOwnerCalibrator))
  ;[1 1 1] Reattach calibration tracker to skeleton and update calibration
  (if (Math|Boolean|ANDBoolean CanUpdateBone (Utilities|Name|NotEqual(Name) (Variables|Default|GetNewBoneName) (Variables|Default|GetBone)) (Utilities|Name|NotEqual(Name) (Variables|Default|GetNewBoneName) "None"))
    (bind _output_get (Variables|Default|SetBone (Variables|Default|GetNewBoneName)))
    (bind _returnvalue (Class|CaptureDevice|UpdateTrackerBone CapDevice (Variables|Default|GetIndex) _output_get))
    (Rendering|Components|TextRender|SetText (Variables|Default|GetTX_Bone) (Utilities|Text|ToText(Name) (Class|CaptureDevice|BonetoName CapDevice _returnvalue))))
  (Utilities|IsValid _ownercalibrator
    (:Is%20Valid
      (Transformation|AttachComponentToComponent self (Variables|/Game/VMK/Blueprints/BP_ManualCalibration.BP_ManualCalibration_C|GetSkeletalMesh _ownercalibrator) (Variables|Default|GetBone) "KeepWorld" "KeepWorld" "KeepWorld" true))
    (:Is%20Not%20Valid
      _))
  (Utilities|FlowControl|Delay 0.1)
  (Class|CaptureDevice|UpdateTrackerTransform CapDevice (Variables|Default|GetIndex) (Math|Transform|InvertTransform (Transformation|GetRelativeTransform (Variables|Transformation|GetRootComponent self)))))

(event EventBeginPlay
  ;[1 1 1] Basic Setup
  (Utilities|Time|SetTimerbyFunctionName 0 "UpdateLabel" 1.0 true)
  (Utilities|FlowControl|Delay 0.4)
  (if (Variables|Settings|GetKeyboardControl)
    (bind _asbp_player_spectator_2d (Utilities|Casting|CastToBP_PlayerSpectator2D (Game|Player|GetPlayerPawn 0)))
    (Variables|Default|SetCapDevice (Variables|/Game/VMK/Blueprints/BP_CapturePawn2D.BP_CapturePawn2D_C|GetCaptureDevice (Variables|/Game/VMK/Blueprints/BP_PlayerSpectator2D.BP_PlayerSpectator2D_C|GetCapturePawn _asbp_player_spectator_2d)))))

(event EventDestroyed
  (bind _currentmanipulator (Variables|Default|GetCurrentManipulator))
  ;[1 1 1] Actions on Deactivate: destroy manipulator, mark as unselected
  (Utilities|IsValid _currentmanipulator
    (:Is%20Valid
      (Actor|DestroyActor _currentmanipulator))
    (:Is%20Not%20Valid
      _))
  (Variables|Settings|SetKeyboardSelected false)
  (Rendering|SetRenderCustomDepth (Variables|Default|GetStaticMesh) false))

(fn ConstructionScript)