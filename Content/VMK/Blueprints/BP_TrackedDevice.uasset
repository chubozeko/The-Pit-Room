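; BP_TrackedDevice is an actor that represents a SteamVR tracked device in the VMK system as a controller or tracker mesh.
; The construction script picks the mesh from the device type.
; Each tick moves the root to the device's tracked pose, raised by a floor offset.
; BeginPlay defaults a negative VMK device ID to the SteamVR ID, and a selection event toggles emissive glow through a dynamic material.
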(event Custom|SetActorSelected
  (params (bIsSelected :type Boolean))
  (Utilities|IsValid (Variables|Default|GetMeshMaterial)
    (:Is%20Valid
      _)
    (:Is%20Not%20Valid
      (bind _returnvalue (Rendering|Material|CreateDynamicMaterialInstance (Variables|Default|GetStaticMesh) 0 0 "None" :!class /Script/Engine.PrimitiveComponent))
      (Variables|Default|SetMeshMaterial _returnvalue)))
  (Rendering|Material|SetScalarParameterValue (Variables|Default|GetMeshMaterial) "EmissionPower" (select bIsSelected 5.0 0.0) :!class /Script/Engine.MaterialInstanceDynamic))

(event EventBeginPlay
  (if (< (Variables|Default|GetVMK_DeviceId) 0)
    (Variables|Default|SetVMK_DeviceId (Variables|Default|GetSteamVR_DeviceId))))

(event EventTick
  (params (DeltaSeconds :type Float%20%28single-precision%29))
  (bind _steamvr_deviceid (Variables|Default|GetSteamVR_DeviceId))
  (bind (_outposition _outorientation) (Class|SteamVRFunctionLibrary|GetTrackedDevicePositionandOrientation _steamvr_deviceid))
  (Transformation|SetRelativeLocationAndRotation (Variables|Default|GetDefaultSceneRoot) (Math|Vector|MakeVector (.x _outposition) (.y _outposition) (+ (.z _outposition) (Variables|Default|GetFloorOffset))) _outorientation false false))

(fn ConstructionScript
  (bind _staticmesh (Variables|Default|GetStaticMesh))
  (bind _staticmesh_2 (Variables|Default|GetStaticMesh))
  (switch Utilities|FlowControl|Switch|SwitchonESteamVRTrackedDeviceType (Variables|Default|GetDeviceType)
    (:Controller
      (Components|StaticMesh|SetStaticMesh _staticmesh "/Game/VMK/StaticMeshes/M_ViveController.M_ViveController")
      (Transformation|SetRelativeRotation _staticmesh_2 "0, 0, 0" false false))
    (:Other
      (Components|StaticMesh|SetStaticMesh _staticmesh "/Game/VMK/StaticMeshes/M_Tracker.M_Tracker")
      (Transformation|SetRelativeRotation _staticmesh_2 "0, 0, 0" false false)
      (Rendering|Material|SetMaterial (Variables|Default|GetStaticMesh) 0 "/Game/VMK/StaticMeshes/M_MetalBlack.M_MetalBlack"))))