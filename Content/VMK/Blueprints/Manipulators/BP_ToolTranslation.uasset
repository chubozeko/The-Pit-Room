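; Translation gizmo that lets the user drag the actor it is attached to along one axis.
; Hovering an axis box highlights it through material parameters; clicking starts Tick and disables pawn input until release.
; Tick projects mouse movement onto the axis's screen direction, scaling it into a filtered world offset for the parent, or only BodyMesh for BP_CapturePawn2D.
; On release, an attached BP_Tracker updates its calibration.
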(event Custom|BeginMouseOver
  (params (TouchedComponent :type Primitive%20Component%20Object%20Reference))
  ;[1 1 1] Select Axis by Mouse Over
  (if (not (Class|Actor|IsActorTickEnabled))
    (bind _asbox_collision (Utilities|Casting|CastToBoxComponent TouchedComponent))
    (Utilities|UpdateAxis _asbox_collision
      (:Out
        (Variables|Default|SetMouseOver true)))))

(event Custom|StopMovement
  (bind _rootcomponent (Variables|Transformation|GetRootComponent))
  (bind _returnvalue (Transformation|GetAttachParent _rootcomponent))
  ;[1 1 1] Update Tracker on movement stop
  (Actor|Tick|SetActorTickEnabled false)
  (Utilities|IsValid _returnvalue
    (:Is%20Valid
      (bind _asbp_tracker (Utilities|Casting|CastToBP_Tracker (Components|GetOwner _returnvalue)))
      (Default|UpdateCalibration _asbp_tracker))))

(event Custom|OnMousePressed
  (params (TouchedComponent :type Primitive%20Component%20Object%20Reference) (ButtonPressed :type Key%20Structure :default "None"))
  ;[1 1 1] Activate Movement by Mouse Press/Release
  (if (and (Utilities|IsValid (Variables|Default|GetCurrentAxisBox)) (== ButtonPressed "LeftMouseButton"))
    (CallFunction|SetupScreentoWorld)
    (Actor|Tick|SetActorTickEnabled true)
    (Input|DisableInput (Game|Player|GetPlayerPawn 0) (Game|GetPlayerController 0))))

(event Custom|OnMouseReleased
  (params (TouchedComponent :type Primitive%20Component%20Object%20Reference) (ButtonReleased :type Key%20Structure :default "None"))
  ;[1 1 1] Activate Movement by Mouse Press/Release
  (if (== ButtonReleased "LeftMouseButton")
    (CallFunction|StopMovement)
    (if (not (Variables|Default|GetMouseOver))
      (Utilities|UpdateAxis
        (:Out
          _)))
    (Input|EnableInput (Game|Player|GetPlayerPawn 0) (Game|GetPlayerController 0))))

(event Custom|EndMouseOver
  (params (TouchedComponent :type Primitive%20Component%20Object%20Reference))
  ;[1 1 1] Select Axis by Mouse Over
  (if (== TouchedComponent (Variables|Default|GetCurrentAxisBox))
    (Variables|Default|SetMouseOver false)
    (if (not (Class|Actor|IsActorTickEnabled))
      (Utilities|UpdateAxis))))

(event Custom|PerformAction
  (params (Target :type Actor%20Object%20Reference) (Value :type Float%20%28single-precision%29))
  ;[1 1 1] Main Action
  (bind _result (Utilities|GetVectorOffset Value)
    (:Out
      (bind _asbp_capture_pawn_2d (Utilities|Casting|CastToBP_CapturePawn2D Target)
        (:then
          (Transformation|AddWorldOffset (Variables|/Game/VMK/Blueprints/BP_CapturePawn2D.BP_CapturePawn2D_C|GetBodyMesh _asbp_capture_pawn_2d) (* _result (Variables|Default|GetActionFilter)) false false))
        (:CastFailed
          (Transformation|AddActorWorldOffset Target (* _result (Variables|Default|GetActionFilter))))))))

(event EventBeginPlay
  ;[1 1 1] Begin Play: Init Material and bind events
  (bind _returnvalue (Rendering|Material|CreateDynamicMaterialInstance (Variables|Debug|GetStaticMeshComponent) 0 0 "None" :!class /Script/Engine.PrimitiveComponent))
  (Variables|Default|SetM_Manipulator _returnvalue)
  (EventDispatchers|BindEventtoOnBeginCursorOver (Variables|Default|GetBoxX) (EventDispatchers|CreateEvent :!event Custom|BeginMouseOver))
  (EventDispatchers|BindEventtoOnEndCursorOver (Variables|Default|GetBoxX) (EventDispatchers|CreateEvent :!event Custom|EndMouseOver))
  (EventDispatchers|BindEventtoOnClicked (Variables|Default|GetBoxX) (EventDispatchers|CreateEvent :!event Custom|OnMousePressed)))

(event EventTick
  (params (DeltaSeconds :type Float%20%28single-precision%29))
  (bind _rootcomponent (Variables|Transformation|GetRootComponent))
  (bind _returnvalue (Transformation|GetAttachParent _rootcomponent))
  ;[1 1 1] Tick: Move Parent
  ;[1 1 1] Stop Movement at LMB Release
  (if (Class|PlayerController|WasInputKeyJustReleased (Game|GetPlayerController 0) "LeftMouseButton")
    (CallFunction|OnMouseReleased 0 "LeftMouseButton")
    (else
      (bind _returnvalue_2 (Class|WidgetLayoutLibrary|GetMousePositiononViewport))
      (bind _output_get (Variables|Default|SetNewMousePos _returnvalue_2))
      (if (> (Math|Vector2D|Vector2DLength (- _output_get (Variables|Default|GetLastMousePos))) 4.0)
        ;[1 1 1] Update Last Coord
        (Utilities|IsValid _returnvalue
          (:Is%20Valid
            (CallFunction|PerformAction (Components|GetOwner _returnvalue) (* (Variables|Default|GetScreenScale) (* (Math|Vector2D|Vector2DLength (- _output_get (Variables|Default|GetLastMousePos))) (Math|Vector2D|DotProduct(2D) (Variables|Default|GetOnScreenDirection) (Math|Vector2D|Normalize2D (- (Variables|Default|GetNewMousePos) (Variables|Default|GetLastMousePos))))))))
          (:Is%20Not%20Valid
            _))
        (Variables|Default|SetLastMousePos (Variables|Default|GetNewMousePos))))))

(fn ConstructionScript)

(fn SetupScreentoWorld
  (bind _returnvalue (Game|GetPlayerController 0))
  (bind _staticmeshcomponent (Variables|Debug|GetStaticMeshComponent))
  (bind _currentaxisbox (Variables|Default|GetCurrentAxisBox))
  (bind _returnvalue_2 (Transformation|GetWorldLocation _currentaxisbox))
  (bind _returnvalue_3 (Transformation|GetWorldLocation _staticmeshcomponent))
  (bind _screenposition (Class|GameplayStatics|ProjectWorldtoScreen _returnvalue _returnvalue_2 false))
  (bind _screenposition_2 (Class|GameplayStatics|ProjectWorldtoScreen _returnvalue _returnvalue_3 false))
  (bind _returnvalue_4 (- _screenposition _screenposition_2))
  (bind _returnvalue_5 (Class|WidgetLayoutLibrary|GetMousePositiononViewport))
  (Variables|Default|SetLastMousePos _returnvalue_5)
  (Variables|Default|SetOnScreenDirection (Math|Vector2D|Normalize2D _returnvalue_4))
  (Variables|Default|SetScreenScale (/ (.z (Variables|/Script/Engine.BoxComponent|GetBoxExtent (Variables|Default|GetBoxY))) (Math|Vector2D|Vector2DLength _returnvalue_4)))
  (return))