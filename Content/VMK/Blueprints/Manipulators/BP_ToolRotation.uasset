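; Rotation gizmo that turns the actor it is attached to by mouse dragging one of three axis handles.
; Hover highlights an axis through a dynamic material; left press disables pawn input and enables Tick until release.
; Tick projects mouse movement onto the axis's screen-space direction, applying filtered local or world rotation, or rotating BP_CapturePawn2D's BodyMesh.
; On release, it restores input and updates calibration on a parent BP_Tracker.
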(event Custom|BeginMouseOver
  (params (TouchedComponent :type Primitive%20Component%20Object%20Reference))
  ;[1 1 1] Select Axis by Mouse Over
  (if (not (Class|Actor|IsActorTickEnabled))
    (Utilities|UpdateAxis TouchedComponent
      (:Out
        (Variables|Default|SetMouseOver true)))))

(event Custom|StopMovement
  (bind _rootcomponent (Variables|Transformation|GetRootComponent))
  (bind _returnvalue (Transformation|GetAttachParent _rootcomponent))
  ;[1 1 1] Update Tracker on movement stop
  (Actor|Tick|SetActorTickEnabled false)
  (Utilities|IsValid _returnvalue
    (:Is%20Valid
      (bind _asbp_tracker (Utilities|Casting|CastToBP_Tracker (Components|GetOwner _returnvalue)))
      (Default|UpdateCalibration _asbp_tracker))))

(event Custom|OnMousePressed
  (params (TouchedComponent :type Primitive%20Component%20Object%20Reference) (ButtonPressed :type Key%20Structure :default "None"))
  ;[1 1 1] Activate Movement by Mouse Press/Release
  (if (and (Utilities|IsValid (Variables|Default|GetCurrentAxisMesh)) (== ButtonPressed "LeftMouseButton"))
    (Utilities|InitScreenDirection
      (:Out
        (Actor|Tick|SetActorTickEnabled true)
        (Input|DisableInput (Game|Player|GetPlayerPawn 0) (Game|GetPlayerController 0))))))

(event Custom|OnMouseReleased
  (params (TouchedComponent :type Primitive%20Component%20Object%20Reference) (ButtonReleased :type Key%20Structure :default "None"))
  ;[1 1 1] Activate Movement by Mouse Press/Release
  (if (== ButtonReleased "LeftMouseButton")
    (CallFunction|StopMovement)
    (if (not (Variables|Default|GetMouseOver))
      (Utilities|UpdateAxis
        (:Out
          _)))
    (Input|EnableInput (Game|Player|GetPlayerPawn 0) (Game|GetPlayerController 0))))

(event Custom|EndMouseOver
  (params (TouchedComponent :type Primitive%20Component%20Object%20Reference))
  ;[1 1 1] Select Axis by Mouse Over
  (if (== TouchedComponent (Variables|Default|GetCurrentAxisMesh))
    (Variables|Default|SetMouseOver false)
    (if (not (Class|Actor|IsActorTickEnabled))
      (Utilities|UpdateAxis))))

(event Custom|PerformAction
  (params (Target :type Actor%20Object%20Reference) (Value :type Float%20%28single-precision%29))
  ;[1 1 1] Perform Rotation
  (bind _result (Utilities|GetRotationOffset Value)
    (:Out
      (bind _asbp_capture_pawn_2d (Utilities|Casting|CastToBP_CapturePawn2D Target)
        (:then
          (Transformation|AddLocalRotation (Variables|/Game/VMK/Blueprints/BP_CapturePawn2D.BP_CapturePawn2D_C|GetBodyMesh _asbp_capture_pawn_2d) _result false false))
        (:CastFailed
          (if (Variables|Default|GetbIsLocal)
            (Transformation|AddActorLocalRotation Target _result false false)
            (else
              (Class|Actor|AddActorWorldRotation Target _result))))))))

(event EventBeginPlay
  ;[1 1 1] Begin Play: Init Material and bind events
  (bind _returnvalue (Rendering|Material|CreateDynamicMaterialInstance (Variables|Debug|GetStaticMeshComponent) 0 0 "None" :!class /Script/Engine.PrimitiveComponent))
  (Variables|Default|SetM_Manipulator _returnvalue)
  (EventDispatchers|BindEventtoOnBeginCursorOver (Variables|Default|GetRotX) (EventDispatchers|CreateEvent :!event Custom|BeginMouseOver))
  (EventDispatchers|BindEventtoOnEndCursorOver (Variables|Default|GetRotX) (EventDispatchers|CreateEvent :!event Custom|EndMouseOver))
  (EventDispatchers|BindEventtoOnClicked (Variables|Default|GetRotX) (EventDispatchers|CreateEvent :!event Custom|OnMousePressed)))

(event EventTick
  (params (DeltaSeconds :type Float%20%28single-precision%29))
  (bind _rootcomponent (Variables|Transformation|GetRootComponent))
  (bind _returnvalue (Transformation|GetAttachParent _rootcomponent))
  ;[1 1 1] Tick: Move Parent
  ;[1 1 1] Stop Movement at LMB Release
  (if (Class|PlayerController|WasInputKeyJustReleased (Game|GetPlayerController 0) "LeftMouseButton")
    (CallFunction|OnMouseReleased 0 "LeftMouseButton")
    (else
      (bind _returnvalue_2 (Class|WidgetLayoutLibrary|GetMousePositiononViewport))
      (bind _output_get (Variables|Default|SetNewMousePos _returnvalue_2))
      (if (> (Math|Vector2D|Vector2DLength (- _output_get (Variables|Default|GetLastMousePos))) 4.0)
        ;[1 1 1] Rotate Object
        (Utilities|IsValid _returnvalue
          (:Is%20Valid
            (CallFunction|PerformAction (Components|GetOwner _returnvalue) (* (Variables|Default|GetScreenScale) (* (Math|Vector2D|Vector2DLength (- _output_get (Variables|Default|GetLastMousePos))) (Math|Vector2D|DotProduct(2D) (Variables|Default|GetOnScreenDirection) (Math|Vector2D|Normalize2D (- (Variables|Default|GetNewMousePos) (Variables|Default|GetLastMousePos)))))))
            ;[1 1 1] Update Last Coord
            (Variables|Default|SetLastMousePos (Variables|Default|GetNewMousePos))))))))

(fn ConstructionScript)