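; Scale manipulator tool that resizes the body mesh of a BP_CapturePawn2D along a selected axis handle.
; SetupScreentoWorld stores the mouse position and projects the handle's axis to screen space, deriving a drag direction and screen-to-world factor.
; PerformAction maps the handle's component tag to an axis, applies the incoming value through ActionFilter as a relative multiplier, clamps each component to a narrow range, and resets the tool's own scale.
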(event EventBeginPlay
  (|CallParentFunction))

(event Collision|EventActorBeginOverlap
  (params (OtherActor :type Actor%20Object%20Reference)))

(event EventTick
  (params (DeltaSeconds :type Float%20%28single-precision%29))
  (|CallParentFunction DeltaSeconds))

(event EventSetupScreentoWorld
  (bind _returnvalue (Game|GetPlayerController 0))
  (bind _staticmeshcomponent (Variables|Default|GetStaticMeshComponent))
  (bind _currentaxisbox (Variables|Default|GetCurrentAxisBox))
  (bind _returnvalue_2 (Transformation|GetWorldLocation _currentaxisbox))
  (bind _returnvalue_3 (Transformation|GetWorldLocation _staticmeshcomponent))
  (bind _screenposition (Class|GameplayStatics|ProjectWorldtoScreen _returnvalue _returnvalue_2 false))
  (bind _screenposition_2 (Class|GameplayStatics|ProjectWorldtoScreen _returnvalue _returnvalue_3 false))
  (bind _returnvalue_4 (- _screenposition _screenposition_2))
  ;[1 1 1] Init for scaling
  ;;[0 0 0] Save Initial Mouse Position
  (bind _returnvalue_5 (Class|WidgetLayoutLibrary|GetMousePositiononViewport))
  (Variables|Default|SetLastMousePos _returnvalue_5)
  (Variables|Default|SetOnScreenDirection (Math|Vector2D|Normalize2D _returnvalue_4))
  ;;[0 0 0] World-to-Screen Scale
  (Variables|Default|SetScreenScale (* (/ (.y (Variables|/Script/Engine.SceneComponent|GetRelativeLocation (Variables|Default|GetBoxY))) (Math|Vector2D|Vector2DLength _returnvalue_4)) 0.1)))

(event EventPerformAction
  (params (Target :type Actor%20Object%20Reference) (Value :type Float%20%28single-precision%29))
  ;[1 1 1] Scale Mesh
  (bind _asbp_capture_pawn_2d (Utilities|Casting|CastToBP_CapturePawn2D Target))
  (Transformation|SetRelativeScale3D (Variables|/Game/VMK/Blueprints/BP_CapturePawn2D.BP_CapturePawn2D_C|GetBodyMesh _asbp_capture_pawn_2d) (Math|Vector|MakeVector (Math|Float|Clamp(Float) (.x (* (Variables|/Script/Engine.SceneComponent|GetRelativeScale3D (Variables|/Game/VMK/Blueprints/BP_CapturePawn2D.BP_CapturePawn2D_C|GetBodyMesh _asbp_capture_pawn_2d)) (+ (* (Utilities|Select :Index (select (Utilities|IsValid (Variables|Default|GetCurrentAxisBox)) (Math|Conversions|ToInteger(Byte) (Utilities|String|ToString(Name) (Utilities|Array|Get(acopy) (Variables|/Script/Engine.ActorComponent|GetComponentTags (Variables|Default|GetCurrentAxisBox))))) 0) :Option%200 "1.000000,1.000000,1.000000" :Option%201 (Math|Vector|MakeVector Value 0.0 0.0) :Option%202 (Math|Vector|MakeVector 0.0 Value 0.0) :Option%203 (Math|Vector|MakeVector 0.0 0.0 Value)) (Variables|Default|GetActionFilter)) "1.000000,1.000000,1.000000"))) 0.6 1.4) (Math|Float|Clamp(Float) (.y (* (Variables|/Script/Engine.SceneComponent|GetRelativeScale3D (Variables|/Game/VMK/Blueprints/BP_CapturePawn2D.BP_CapturePawn2D_C|GetBodyMesh _asbp_capture_pawn_2d)) (+ (* (Utilities|Select :Index (select (Utilities|IsValid (Variables|Default|GetCurrentAxisBox)) (Math|Conversions|ToInteger(Byte) (Utilities|String|ToString(Name) (Utilities|Array|Get(acopy) (Variables|/Script/Engine.ActorComponent|GetComponentTags (Variables|Default|GetCurrentAxisBox))))) 0) :Option%200 "1.000000,1.000000,1.000000" :Option%201 (Math|Vector|MakeVector Value 0.0 0.0) :Option%202 (Math|Vector|MakeVector 0.0 Value 0.0) :Option%203 (Math|Vector|MakeVector 0.0 0.0 Value)) (Variables|Default|GetActionFilter)) "1.000000,1.000000,1.000000"))) 0.6 1.4) (Math|Float|Clamp(Float) (.z (* (Variables|/Script/Engine.SceneComponent|GetRelativeScale3D (Variables|/Game/VMK/Blueprints/BP_CapturePawn2D.BP_CapturePawn2D_C|GetBodyMesh _asbp_capture_pawn_2d)) (+ (* (Utilities|Select :Index (select (Utilities|IsValid (Variables|Default|GetCurrentAxisBox)) (Math|Conversions|ToInteger(Byte) (Utilities|String|ToString(Name) (Utilities|Array|Get(acopy) (Variables|/Script/Engine.ActorComponent|GetComponentTags (Variables|Default|GetCurrentAxisBox))))) 0) :Option%200 "1.000000,1.000000,1.000000" :Option%201 (Math|Vector|MakeVector Value 0.0 0.0) :Option%202 (Math|Vector|MakeVector 0.0 Value 0.0) :Option%203 (Math|Vector|MakeVector 0.0 0.0 Value)) (Variables|Default|GetActionFilter)) "1.000000,1.000000,1.000000"))) 0.6 1.4)))
  (Transformation|SetActorScale3D "1.000000,1.000000,1.000000"))

(fn ConstructionScript
  (|CallParentFunction))