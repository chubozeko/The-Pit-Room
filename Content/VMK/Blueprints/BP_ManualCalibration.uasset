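; Manual calibration actor for motion capture trackers, assigning them to skeleton bones through per-bone capsule colliders on a skeletal mesh.
; It spawns BP_Tracker actors from CaptureDevice data, and capsule overlaps set each tracker's new bone after conflict checks.
; Overlapping BP_TrackedDevice actors toggle highlight spheres and broadcast an overlap count.
; Without HMD head tracking, it plays a T-pose, enables tracker keyboard control and supports limiting colliders to active bones.
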(event Custom|DestroyMe
  ;[1 1 1] Kill all trackers on destroy
  (for _array_element (Variables|Default|GetTrackers)
    (Actor|DestroyActor _array_element))
  (CallFunction|DestroyAllSpheres)
  (Actor|DestroyActor))

(event Custom|UpdateCollidersFor2D
  (params (ActiveBones :type Set%20of%20EHumanoidBone%20Enums :default "Root"))
  ;[1 1 1] Disable collision for inactive bones (for non-HMD map)
  (bind _result (Utilities|Set|ToArray ActiveBones))
  (Utilities|Array|Clear (Variables|Default|GetAllowedColliders))
  (for _array_element _result
    (Utilities|Array|Add (Variables|Default|GetAllowedColliders) (.Value (Utilities|Map|Find (Variables|Default|GetBonesPreset) _array_element))))
  (for _array_element_2 (Variables|Default|GetColliders)
    (Collision|SetCollisionEnabled _array_element_2 (select (Utilities|Array|ContainsItem (Variables|Default|GetAllowedColliders) (Transformation|GetAttachSocketName _array_element_2)) "QueryOnly" "NoCollision"))))

(event Custom|OnTriggerEndOverlap
  (params (OverlappedComponent :type Primitive%20Component%20Object%20Reference) (OtherActor :type Actor%20Object%20Reference) (OtherComp :type Primitive%20Component%20Object%20Reference) (OtherBodyIndex :type Integer))
  ;[1 1 1] Non-HMD map: counting BP_MotionDevice actors in bone colliders
  (Utilities|Casting|CastToBP_TrackedDevice OtherActor)
  (CallFunction|DestroySphere OverlappedComponent)
  (Variables|Default|SetOverlappingDevices 0)
  (for _array_element (Variables|Default|GetColliders)
    (if (Class|PrimitiveComponent|IsCollisionEnabled _array_element)
      (Variables|Default|SetOverlappingDevices (+ (Variables|Default|GetOverlappingDevices) (Utilities|Array|Length (Collision|GetOverlappingActors _array_element "/Game/VMK/Blueprints/BP_TrackedDevice.BP_TrackedDevice_C" :!class /Script/Engine.PrimitiveComponent))))))
  (Default|CallOnMotionDevicesOverlapEvent (Variables|Default|GetOverlappingDevices)))

(event Custom|DestroyAllSpheres
  ;[1 1 1] Non-HMD map: counting BP_MotionDevice actors in bone colliders
  (bind _values (Utilities|Map|Values (Variables|Default|GetHighlightSpheres)))
  (for _array_element _values
    (Utilities|IsValid _array_element
      (:Is%20Valid
        (Actor|DestroyActor _array_element))))
  (Utilities|Map|Clear (Variables|Default|GetHighlightSpheres))
  (Variables|Default|SetbNoSpheres true))

(event Custom|DestroySphere
  (params (Collider :type Primitive%20Component%20Object%20Reference))
  (bind _returnvalue (Transformation|GetAttachSocketName Collider))
  (bind _highlightspheres (Variables|Default|GetHighlightSpheres))
  (bind (_value _returnvalue_2) (Utilities|Map|Find _highlightspheres _returnvalue))
  ;[1 1 1] Non-HMD map: counting BP_MotionDevice actors in bone colliders
  (if _returnvalue_2
    (Utilities|IsValid _value
      (:Is%20Valid
        (Actor|DestroyActor _value)
        (Utilities|Map|Remove (Variables|Default|GetHighlightSpheres) _returnvalue)))))

(event Custom|OnTriggerBeginOverlap
  (params (OverlappedComponent :type Primitive%20Component%20Object%20Reference) (OtherActor :type Actor%20Object%20Reference) (OtherComp :type Primitive%20Component%20Object%20Reference) (OtherBodyIndex :type Integer) (bFromSweep :type Boolean) (SweepResult :type Hit%20Result%20Structure%20%28by%20ref%29))
  (bind _returnvalue (Transformation|GetAttachSocketName OverlappedComponent))
  ;[1 1 1] Update target bone name of a tracker
  (bind _asbp_tracker (Utilities|Casting|CastToBP_Tracker OtherActor)
    (:then
      (if (or (!= OverlappedComponent (Variables|Default|GetCapsule16)) (Variables|Default|GetMode2D))
        (Utilities|FlowControl|Sequence
          (:then_0
            (Utilities|CheckRibcageCollar _asbp_tracker _returnvalue
              (:CanBeChanged
                (Utilities|CheckCalfFoot _asbp_tracker _returnvalue
                  (:CanBeChanged
                    (Variables|Default|SetIgnoreOverlap false)
                    (|CheckExistingTracker _asbp_tracker _returnvalue
                      (:Completed
                        (if (not (Variables|Default|GetIgnoreOverlap))
                          (Variables|/Game/VMK/Blueprints/BP_Tracker.BP_Tracker_C|SetNewBoneName _asbp_tracker _returnvalue))))))))))))
    (:CastFailed
      ;[1 1 1] Non-HMD map: counting BP_MotionDevice actors in bone colliders
      (Utilities|Casting|CastToBP_TrackedDevice OtherActor)
      (CallFunction|SpawnSphere OverlappedComponent)
      (Variables|Default|SetOverlappingDevices 0)
      (for _array_element (Variables|Default|GetColliders)
        (if (Class|PrimitiveComponent|IsCollisionEnabled _array_element)
          (Variables|Default|SetOverlappingDevices (+ (Variables|Default|GetOverlappingDevices) (Utilities|Array|Length (Collision|GetOverlappingActors _array_element "/Game/VMK/Blueprints/BP_TrackedDevice.BP_TrackedDevice_C" :!class /Script/Engine.PrimitiveComponent))))))
      (Default|CallOnMotionDevicesOverlapEvent (Variables|Default|GetOverlappingDevices)))))

(event Custom|SpawnSphere
  (params (Collider :type Primitive%20Component%20Object%20Reference))
  ;[1 1 1] Non-HMD map: counting BP_MotionDevice actors in bone colliders
  (if (not (Variables|Default|GetbNoSpheres))
    (CallFunction|DestroySphere Collider)
    (bind _returnvalue (Game|SpawnActorfromClass "/Game/VMK/Blueprints/BP_Highlight.BP_Highlight_C" (Transformation|GetWorldTransform Collider) "Undefined" 0 0))
    (Utilities|Map|Add (Variables|Default|GetHighlightSpheres) (Transformation|GetAttachSocketName Collider) _returnvalue)))

(event EventBeginPlay
  (bind _capturedevice (Variables|References|GetCaptureDevice))
  (bind _output_get (Variables|Default|SetColliders (Utilities|Array|MakeArray (Variables|Default|GetCapsule0) (Variables|Default|GetCapsule1) (Variables|Default|GetCapsule2) (Variables|Default|GetCapsule3) (Variables|Default|GetCapsule4) (Variables|Default|GetCapsule5) (Variables|Default|GetCapsule6) (Variables|Default|GetCapsule7) (Variables|Default|GetCapsule8) (Variables|Default|GetCapsule9) (Variables|Default|GetCapsule10) (Variables|Default|GetCapsule11) (Variables|Default|GetCapsule12) (Variables|Default|GetCapsule13) (Variables|Default|GetCapsule14) (Variables|Default|GetCapsule15) (Variables|Default|GetCapsule16))))
  (for _array_element _output_get
    (Collision|BindEventtoOnComponentBeginOverlap _array_element (delegate Custom|OnTriggerBeginOverlap))
    (Collision|BindEventtoOnComponentEndOverlap _array_element (delegate Custom|OnTriggerEndOverlap)))
  (Utilities|FlowControl|Delay 0.2)
  (Utilities|IsValid _capturedevice
    (:Is%20Valid
      (bind _output_get_2 (Variables|Default|SetMode2D (not (Variables|/Script/ViveMocapKit.CaptureDevice|GetbUseVRHeadsetForHead _capturedevice))))
      (Rendering|SetVisibility (Variables|Default|GetStaticMesh) (not _output_get_2) false)
      (Variables|Default|SetTrackerHands (Utilities|Enum|Equal(Enum) (Variables|/Script/ViveMocapKit.CaptureDevice|GetMotionControllersTrackingRole _capturedevice) "HandsOnly"))
      (if (Variables|Default|GetMode2D)
        ;[1 1 1] For Non-HMD map: set T-Pose animation
        (Components|Animation|SetAnimation (Variables|Default|GetSkeletalMesh) (Variables|Default|GetTPose_Animation)))
      (|SpawnBP_Trackercomponents))))

(fn ConstructionScript
  (Transformation|AttachComponentToComponent (Variables|Default|GetCapsule0) (Variables|Default|GetSkeletalMesh) (Utilities|BoneName "UpperarmLeft") "KeepRelative" "KeepRelative" "KeepRelative" true)
  (Transformation|AttachComponentToComponent (Variables|Default|GetCapsule1) (Variables|Default|GetSkeletalMesh) (Utilities|BoneName "ForearmLeft") "KeepRelative" "KeepRelative" "KeepRelative" true)
  (Transformation|AttachComponentToComponent (Variables|Default|GetCapsule2) (Variables|Default|GetSkeletalMesh) (Utilities|BoneName "PalmLeft") "KeepRelative" "KeepRelative" "KeepRelative" true)
  (Transformation|AttachComponentToComponent (Variables|Default|GetCapsule3) (Variables|Default|GetSkeletalMesh) (Utilities|BoneName "ShoulderLeft") "KeepRelative" "KeepRelative" "KeepRelative" true)
  (Transformation|AttachComponentToComponent (Variables|Default|GetCapsule4) (Variables|Default|GetSkeletalMesh) (Utilities|BoneName "ShoulderRight") "KeepRelative" "KeepRelative" "KeepRelative" true)
  (Transformation|AttachComponentToComponent (Variables|Default|GetCapsule5) (Variables|Default|GetSkeletalMesh) (Utilities|BoneName "UpperarmRight") "KeepRelative" "KeepRelative" "KeepRelative" true)
  (Transformation|AttachComponentToComponent (Variables|Default|GetCapsule6) (Variables|Default|GetSkeletalMesh) (Utilities|BoneName "ForearmRight") "KeepRelative" "KeepRelative" "KeepRelative" true)
  (Transformation|AttachComponentToComponent (Variables|Default|GetCapsule7) (Variables|Default|GetSkeletalMesh) (Utilities|BoneName "PalmRight") "KeepRelative" "KeepRelative" "KeepRelative" true)
  (Transformation|AttachComponentToComponent (Variables|Default|GetCapsule8) (Variables|Default|GetSkeletalMesh) (Utilities|BoneName "Ribcage") "KeepRelative" "KeepRelative" "KeepRelative" true)
  (Transformation|AttachComponentToComponent (Variables|Default|GetCapsule9) (Variables|Default|GetSkeletalMesh) (Utilities|BoneName "Pelvis") "KeepRelative" "KeepRelative" "KeepRelative" true)
  (Transformation|AttachComponentToComponent (Variables|Default|GetCapsule10) (Variables|Default|GetSkeletalMesh) (Utilities|BoneName "ThighLeft") "KeepRelative" "KeepRelative" "KeepRelative" true)
  (Transformation|AttachComponentToComponent (Variables|Default|GetCapsule11) (Variables|Default|GetSkeletalMesh) (Utilities|BoneName "ThighRight") "KeepRelative" "KeepRelative" "KeepRelative" true)
  (Transformation|AttachComponentToComponent (Variables|Default|GetCapsule12) (Variables|Default|GetSkeletalMesh) (Utilities|BoneName "CalfLeft") "KeepRelative" "KeepRelative" "KeepRelative" true)
  (Transformation|AttachComponentToComponent (Variables|Default|GetCapsule13) (Variables|Default|GetSkeletalMesh) (Utilities|BoneName "CalfRight") "KeepRelative" "KeepRelative" "KeepRelative" true)
  (Transformation|AttachComponentToComponent (Variables|Default|GetCapsule14) (Variables|Default|GetSkeletalMesh) (Utilities|BoneName "FootLeft") "KeepRelative" "KeepRelative" "KeepRelative" true)
  (Transformation|AttachComponentToComponent (Variables|Default|GetCapsule15) (Variables|Default|GetSkeletalMesh) (Utilities|BoneName "FootRight") "KeepRelative" "KeepRelative" "KeepRelative" true)
  (Transformation|AttachComponentToComponent (Variables|Default|GetCapsule16) (Variables|Default|GetSkeletalMesh) (Utilities|BoneName "Head") "KeepRelative" "KeepRelative" "KeepRelative" true))