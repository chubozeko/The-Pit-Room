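; Scene component that follows a VR tracked device, either a left or right controller or a tracker chosen by Hand.
; It resolves the device ID by motion source, re-querying on a looping timer until the ID is valid and an update window expires.
; Tick copies the device pose to its relative transform, or resets it without a device.
; It also picks a Vive controller or tracker mesh and highlights an attached mesh through emissive material when selected.
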(event Custom|UpdateDeviceId
  (if (or (< (Variables|Default|GetTrackerId) 0) (< (Utilities|Time|GetRealTimeSeconds) (Variables|Default|GetEndUpdateIdTime)))
    (bind _returnvalue (Class|SteamVRTrackingLibBPLibrary|GetDeviceIdbyMotionSource (Utilities|HandtoMotionSource (Variables|Default|GetHand)) false (Utilities|GetDeviceType)))
    (Variables|Default|SetTrackerId _returnvalue)
    (else
      (Utilities|Time|ClearandInvalidateTimerbyHandle (Variables|Default|GetTimer_UpdateDeviceId)))))

(event Custom|SetComponentSelected
  (params (bIsSelected :type Boolean))
  (bind _childmeshcomponent (Variables|Default|GetChildMeshComponent))
  (Utilities|IsValid _childmeshcomponent
    (:Is%20Valid
      (Utilities|IsValid (Variables|Default|GetMeshMaterial)
        (:Is%20Valid
          _)
        (:Is%20Not%20Valid
          (bind _returnvalue (Rendering|Material|CreateDynamicMaterialInstance _childmeshcomponent 0 0 "None" :!class /Script/Engine.PrimitiveComponent))
          (Variables|Default|SetMeshMaterial _returnvalue)))
      (Rendering|Material|SetScalarParameterValue (Variables|Default|GetMeshMaterial) "EmissionPower" (select bIsSelected 5.0 0.0) :!class /Script/Engine.MaterialInstanceDynamic))))

(event Custom|InitChildMesh
  (params (AttachedComp :type Static%20Mesh%20Component%20Object%20Reference))
  (Variables|Default|SetChildMeshComponent AttachedComp))

(event EventTick
  (params (DeltaSeconds :type Float%20%28single-precision%29))
  (bind _trackerid (Variables|Default|GetTrackerId))
  (bind (_outposition _outorientation) (Class|SteamVRFunctionLibrary|GetTrackedDevicePositionandOrientation _trackerid))
  (if (>= _trackerid 0)
    (Transformation|SetRelativeLocationAndRotation _outposition _outorientation false false)
    (else
      (Transformation|SetRelativeLocationAndRotation "0, 0, 0" "0, 0, 0" false false))))

(event EventBeginPlay
  (bind _hand (Variables|Default|GetHand))
  (if (Math|Boolean|ORBoolean (Utilities|Enum|Equal(Enum) _hand "Left") (Utilities|Enum|Equal(Enum) _hand "Right") (>= _hand (Variables|Default|GetTrackerHand)))
    (bind _returnvalue (Class|SteamVRTrackingLibBPLibrary|GetDeviceIdbyMotionSource (Utilities|HandtoMotionSource (Variables|Default|GetHand)) false (Utilities|GetDeviceType)))
    (Variables|Default|SetTrackerId _returnvalue)
    (Variables|Default|SetEndUpdateIdTime (+ (Utilities|Time|GetRealTimeSeconds) (Variables|Default|GetUpdateHandIdTime)))
    (bind _returnvalue_2 (Utilities|Time|SetTimerbyFunctionName 0 "UpdateDeviceId" 1.0 true))
    (Variables|Default|SetTimer_UpdateDeviceId _returnvalue_2)))

(fn GetStaticMesh
  (return (select (Utilities|Array|ContainsItem (Class|SteamVRFunctionLibrary|GetValidTrackedDeviceIds "Controller") (Variables|Default|GetTrackerId)) "/Game/VMK/StaticMeshes/M_ViveController.M_ViveController" "/Game/VMK/StaticMeshes/M_Tracker.M_Tracker")))