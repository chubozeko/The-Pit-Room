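; BP_Timer is a record timer actor that shows recording status and elapsed minutes and seconds through text components.
; Shortly after BeginPlay it registers itself as the TimerActor on the player's BP_CapturePawn.
; StartTimer and StopTimer switch a one-second looping timer and the on/off title.
; Each tick of that timer formats the game time elapsed since the stored start time into the display.
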(event Custom|StartTimer
  ;[1 1 1] Enable/Disable Timer
  (Variables|Default|SetBaseTime (Utilities|Time|GetGameTimeinSeconds))
  (Utilities|Time|SetTimerbyFunctionName 0 "OnTimer" 1.0 true)
  (Rendering|Components|TextRender|SetText (Variables|Default|GetT_Title) (Utilities|Text|MakeLiteralText "Record is ON")))

(event Custom|StopTimer
  ;[1 1 1] Enable/Disable Timer
  (Utilities|Time|ClearTimerbyFunctionName 0 "OnTimer")
  (Rendering|Components|TextRender|SetText (Variables|Default|GetT_Title) (Utilities|Text|MakeLiteralText "Record is OFF")))

(event Custom|OnTimer
  (bind _returnvalue (Utilities|Time|GetGameTimeinSeconds))
  (bind _basetime (Variables|Default|GetBaseTime))
  (bind _returnvalue_2 (- _returnvalue _basetime))
  ;[1 1 1] Update Timer Text
  (Rendering|Components|TextRender|SetText (Variables|Default|GetTextRender) (Utilities|Text|FormatText "{mm}:{ss}" (Utilities|Text|ToText(Integer) (Math|Float|Floor (/ _returnvalue_2 6e+01)) false true 2 2) (Utilities|Text|ToText(Float) (Math|Float|%(Float) _returnvalue_2 6e+01) "HalfToEven" false true 2 2 0 0))))

(event EventBeginPlay
  ;[1 1 1] Initialize Player Pawn
  (Utilities|FlowControl|Delay 0.4)
  (bind _asbp_capture_pawn (Utilities|Casting|CastToBP_CapturePawn (Game|Player|GetPlayerPawn 0)))
  (Variables|/Game/VMK/Blueprints/BP_CapturePawn.BP_CapturePawn_C|SetTimerActor _asbp_capture_pawn self))

(fn ConstructionScript)