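; BP_CloneMesh is a clone character actor whose skeletal mesh mirrors the active BP_SkeletonPreset in the level.
; On BeginPlay it finds the first active preset and applies its skeletal mesh and clone Animation Blueprint to SKM.
; It then caches the player's BP_CapturePawn, which this graph does not otherwise use.
; The UpdateClones event reruns the same sequence to refresh the clone.
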(event Custom|Update%20Clones
  (bind _outactors (Actor|GetAllActorsOfClass "/Game/VMK/Blueprints/BP_SkeletonPreset.BP_SkeletonPreset_C"))
  (bind _array_element (Utilities|Array|ForEachLoopwithBreak _outactors :!label _label)
    (:LoopBody
      (if (Variables|/Game/VMK/Blueprints/BP_SkeletonPreset.BP_SkeletonPreset_C|GetIsActive _array_element)
        (Class|SkinnedMeshComponent|SetSkeletalMesh (Variables|Default|GetSKM) (Variables|/Game/VMK/Blueprints/BP_SkeletonPreset.BP_SkeletonPreset_C|GetSkeletalMesh _array_element) true)
        (Class|SkeletalMeshComponent|SetAnimClass (Variables|Default|GetSKM) (Variables|/Game/VMK/Blueprints/BP_SkeletonPreset.BP_SkeletonPreset_C|GetCloneAnimationBlueprint _array_element))
        (goto _label Break)))
    (:Completed
      (bind _asbp_capture_pawn (Utilities|Casting|CastToBP_CapturePawn (Game|Player|GetPlayerPawn 0)))
      (Variables|Default|SetCapturePawn _asbp_capture_pawn))))

(event EventBeginPlay
  (bind _outactors (Actor|GetAllActorsOfClass "/Game/VMK/Blueprints/BP_SkeletonPreset.BP_SkeletonPreset_C"))
  (bind _array_element (Utilities|Array|ForEachLoopwithBreak _outactors :!label _label)
    (:LoopBody
      (if (Variables|/Game/VMK/Blueprints/BP_SkeletonPreset.BP_SkeletonPreset_C|GetIsActive _array_element)
        (Class|SkinnedMeshComponent|SetSkeletalMesh (Variables|Default|GetSKM) (Variables|/Game/VMK/Blueprints/BP_SkeletonPreset.BP_SkeletonPreset_C|GetSkeletalMesh _array_element) true)
        (Class|SkeletalMeshComponent|SetAnimClass (Variables|Default|GetSKM) (Variables|/Game/VMK/Blueprints/BP_SkeletonPreset.BP_SkeletonPreset_C|GetCloneAnimationBlueprint _array_element))
        (goto _label Break)))
    (:Completed
      (bind _asbp_capture_pawn (Utilities|Casting|CastToBP_CapturePawn (Game|Player|GetPlayerPawn 0)))
      (Variables|Default|SetCapturePawn _asbp_capture_pawn))))

(fn ConstructionScript)