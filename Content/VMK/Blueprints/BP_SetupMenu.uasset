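; BP_SetupMenu is an actor that hosts a multi-step calibration setup wizard on a widget component.
; At BeginPlay it passes itself to the initial wizard widget and, after a short delay, registers as the capture pawn's GameMenu.
; Each Show event creates a step widget with a back-reference to the menu and swaps it into the component.
; OnCalibrationLoaded activates the restore-calibration screen's buttons when that screen is showing.
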(event Custom|ShowSetupMenu
  ;[1 1 1] Update Wizard Screen
  (bind _returnvalue (UserInterface|CreateWidget "/Game/VMK/Slate/W_Wizard_02_Setup.W_Wizard_02_Setup_C" (Game|GetPlayerController 0) self))
  (bind _output_get (Variables|Default|SetW%20Wizard%2002%20Setup _returnvalue))
  (UserInterface|SetWidget (Variables|Default|GetWidgetComp) _output_get))

(event Custom|ShowNoHMD_Menu
  ;[1 1 1] Update Wizard Screen
  (bind _returnvalue (UserInterface|CreateWidget "/Game/VMK/Slate/W_Wizard_03A_ForwardCalibration.W_Wizard_03A_ForwardCalibration_C" (Game|GetPlayerController 0) self))
  (UserInterface|SetWidget (Variables|Default|GetWidgetComp) _returnvalue))

(event Custom|ShowLoadCalibration_Menu
  ;[1 1 1] Update Wizard Screen
  (bind _returnvalue (UserInterface|CreateWidget "/Game/VMK/Slate/W_Wizard_03B_RestoreCalibration.W_Wizard_03B_RestoreCalibration_C" (Game|GetPlayerController 0) self))
  (UserInterface|SetWidget (Variables|Default|GetWidgetComp) _returnvalue))

(event Custom|OnCalibrationLoaded
  (bind _asw_wizard_03b_restore_calibration (Utilities|Casting|CastToW_Wizard_03B_RestoreCalibration (UserInterface|GetUserWidgetObject (Variables|Default|GetWidgetComp))))
  (Default|ActivateButtons _asw_wizard_03b_restore_calibration))

(event Custom|ShowAutoCalibrationMenu
  ;[1 1 1] Update Wizard Screen
  (bind _returnvalue (UserInterface|CreateWidget "/Game/VMK/Slate/W_Wizard_03_AutoCalibration.W_Wizard_03_AutoCalibration_C" (Game|GetPlayerController 0) self))
  (bind _output_get (Variables|Default|SetW%20Wizard%2003%20AutoCal _returnvalue))
  (UserInterface|SetWidget (Variables|Default|GetWidgetComp) _output_get)
  (Default|Update _returnvalue))

(event Custom|ShowManualCalibrationMenu
  ;[1 1 1] Update Wizard Screen
  (bind _returnvalue (UserInterface|CreateWidget "/Game/VMK/Slate/W_Wizard_04_ManualCalibration.W_Wizard_04_ManualCalibration_C" (Game|GetPlayerController 0) self))
  (UserInterface|SetWidget (Variables|Default|GetWidgetComp) _returnvalue))

(event Custom|ShowEndMenu
  ;[1 1 1] Update Wizard Screen
  (bind _returnvalue (UserInterface|CreateWidget "/Game/VMK/Slate/W_Wizard_04_Done.W_Wizard_04_Done_C" (Game|GetPlayerController 0) self))
  (UserInterface|SetWidget (Variables|Default|GetWidgetComp) _returnvalue))

(event EventBeginPlay
  ;[1 1 1] Begin Play
  (bind _asw_wizard_01_init (Utilities|Casting|CastToW_Wizard_01_Init (UserInterface|GetUserWidgetObject (Variables|Default|GetWidgetComp))))
  (Variables|/Game/VMK/Slate/W_Wizard_01_Init.W_Wizard_01_Init_C|SetMenu _asw_wizard_01_init self)
  (Utilities|FlowControl|Delay 0.2)
  (bind _asbp_capture_pawn (Utilities|Casting|CastToBP_CapturePawn (Game|Player|GetPlayerPawn 0)))
  (Variables|/Game/VMK/Blueprints/BP_CapturePawn.BP_CapturePawn_C|SetGameMenu _asbp_capture_pawn self))

(fn ConstructionScript)