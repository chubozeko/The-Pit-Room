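; Desktop-menu pawn for full-body motion capture with Vive trackers and motion controllers, recording the performance as animation sequences.
; On start it applies the active BP_SkeletonPreset to the body mesh and CaptureDevice, takes input from an editor trackers controller or SteamVR devices, and spawns tracker actors.
; Wizard widgets drive automatic, manual or saved T-pose calibration.
; It also toggles console-command recording and cycles axis-limited move, rotate and scale gizmos.
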(event Custom|RecalibrateFloorForSpawnedDevices
  (for _array_element (Variables|Default|GetTrackingDevices)
    (Variables|/Game/VMK/Blueprints/BP_TrackedDevice.BP_TrackedDevice_C|SetFloorOffset _array_element (Variables|/Script/ViveMocapKit.CaptureDevice|GetManualFloorOffset (Variables|Default|GetCaptureDevice)))))

(event Custom|New_DoCalibration
  ;[1 1 1] Automatic Calibration
  (Class|CaptureDevice|CalibrateBones (Variables|Default|GetCaptureDevice) false)
  (Rendering|SetVisibility (Variables|Default|GetBodyMesh) true false)
  (|HideCalibrationHelperActors
    (:Completed
      (Variables|CaptureState|SetState "NewEnumerator0")
      (Variables|CaptureState|SetIsCalibrated true)
      (Utilities|FlowControl|Delay 0.2)
      (Class|CaptureDevice|ToggleCapture (Variables|Default|GetCaptureDevice) true false)
      (Utilities|FlowControl|Delay 0.2)
      (for _array_element (Actor|GetComponentsByClass "/Script/HeadMountedDisplay.MotionControllerComponent")
        (bind _returnvalue (AddComponent|AddTextRenderComponent false (Math|Transform|MakeTransform "0,5.000000,0.000000" "0.000000, 0,90.000000")))
        (Transformation|AttachComponentToComponent _returnvalue _array_element "None" "KeepRelative" "KeepRelative" "KeepRelative" true)
        (Rendering|Components|TextRender|SetText _returnvalue (|BuildBoneName _array_element))
        (Rendering|Components|TextRender|SetWorldSize _returnvalue 7.0)
        (Rendering|Components|TextRender|SetHorizontalAlignment _returnvalue "EHTA_Center"))
      (Utilities|IsValid (Variables|References|GetMainMenuWidget)
        (:Is%20Valid
          (Default|OnPlayerCalibratied (Variables|References|GetMainMenuWidget)))))))

(event Custom|InitializeManualCalibrator
  (params (ActiveBones :type Set%20of%20EHumanoidBone%20Enums :default "Root"))
  ;[1 1 1] Only activate colliders for active (selected in the menu) bones
  (bind _returnvalue (Game|SpawnActorfromClass (Variables|Settings|GetManualCalibratorClass) (Transformation|GetWorldTransform (Variables|Default|GetArrow)) "Undefined" 0 (Variables|Default|GetCaptureDevice) 0))
  (bind _output_get (Variables|References|SetManualCalibrator _returnvalue))
  (Default|UpdateCollidersfor2D _output_get ActiveBones)
  (EventDispatchers|BindEventtoOnMotionDevicesOverlapEvent _output_get (delegate Custom|OnMotionDevicesCalibration))
  (Rendering|SetActorHiddenInGame (Variables|References|GetManualCalibrator) true))

(event Custom|RelocateToCenter
  ;[1 1 1] Helpers
  (Variables|Default|SetDeltaTransform (Math|Transform|MakeRelativeTransform (Variables|Default|GetTargetTransform) (|GetCurrentBodyTransform)))
  (Transformation|SetActorTransform (Variables|Default|GetDeltaTransform)))

(event Custom|DoCalibration_Forward
  ;[1 1 1] New calibration process
  (Class|CaptureDevice|PrepareforCalibrationwithHandsForward (Variables|Default|GetCaptureDevice)))

(event Custom|DoCalibration_TPose
  (bind _manualcalibrator (Variables|References|GetManualCalibrator))
  ;[1 1 1] New calibration process
  (Class|CaptureDevice|PrepareforCalibration (Variables|Default|GetCaptureDevice))
  (Rendering|SetActorHiddenInGame _manualcalibrator false)
  (Transformation|SetActorTransform _manualcalibrator (Transformation|GetWorldTransform (Variables|Default|GetBodyMesh)))
  (Rendering|SetVisibility (Variables|Default|GetBodyMesh) false false))

(event Custom|DoAutoCalibration
  ;[1 1 1] Automatic Calibration
  (Class|CaptureDevice|PrepareforCalibration (Variables|Default|GetCaptureDevice))
  (Class|CaptureDevice|CalibrateBones (Variables|Default|GetCaptureDevice) false)
  (Rendering|SetVisibility (Variables|Default|GetBodyMesh) true false)
  (|HideCalibrationHelperActors
    (:Completed
      (Variables|CaptureState|SetState "NewEnumerator0")
      (Variables|CaptureState|SetIsCalibrated true)
      (Utilities|FlowControl|Delay 0.2)
      (Class|CaptureDevice|ToggleCapture (Variables|Default|GetCaptureDevice) true false)
      (Utilities|FlowControl|Delay 0.2)
      (for _array_element (Actor|GetComponentsByClass "/Script/HeadMountedDisplay.MotionControllerComponent")
        (bind _returnvalue (AddComponent|AddTextRenderComponent false (Math|Transform|MakeTransform "0,5.000000,0.000000" "0.000000, 0,90.000000")))
        (Transformation|AttachComponentToComponent _returnvalue _array_element "None" "KeepRelative" "KeepRelative" "KeepRelative" true)
        (Rendering|Components|TextRender|SetText _returnvalue (|BuildBoneName _array_element))
        (Rendering|Components|TextRender|SetWorldSize _returnvalue 7.0)
        (Rendering|Components|TextRender|SetHorizontalAlignment _returnvalue "EHTA_Center"))
      (Utilities|IsValid (Variables|References|GetMainMenuWidget)
        (:Is%20Valid
          (Default|OnPlayerCalibratied (Variables|References|GetMainMenuWidget)))))))

(event Custom|UpdateSkeletonSettings
  ;[1 1 1] Load Settings from BP_SkeletonPreset
  (|ExtractDataFromPreset
    (:Completed
      (Utilities|FlowControl|Delay 0.2)
      (bind _ascapture_anim_blueprint (Utilities|Casting|CastToCaptureAnimBlueprint (Components|SkeletalMesh|GetAnimInstance (Variables|Default|GetBodyMesh))))
      (Variables|/Script/ViveMocapKit.CaptureAnimBlueprint|SetCaptureDevice _ascapture_anim_blueprint (Variables|Default|GetCaptureDevice)))))

(event Custom|SetTrackersVisibility
  (params (bNewVisible :type Boolean))
  ;[1 1 1] Helpers
  (for _array_element (Variables|Default|GetTrackingDevices)
    (Rendering|SetActorHiddenInGame _array_element (not bNewVisible))))

(event Custom|SaveCalibrationPreset
  ;[1 1 1] Save/Load calibration
  (bind _returnvalue (SaveGame|CreateSaveGameObject "/Game/VMK/Blueprints/BP_CalibratonFile.BP_CalibratonFile_C"))
  (bind _outcalibrationdata (Class|CaptureDevice|GetCalibratedDatainTPose (Variables|Default|GetCaptureDevice)))
  (Variables|/Game/VMK/Blueprints/BP_CalibratonFile.BP_CalibratonFile_C|SetNewData _returnvalue _outcalibrationdata)
  (SaveGame|SaveGametoSlot _returnvalue (Variables|Default|GetCalibrationFile))
  (bind _returnvalue_2 (SaveGame|CreateSaveGameObject "/Script/SteamVRTrackingLib.SessionCalibrationSave"))
  (Variables|/Script/SteamVRTrackingLib.SessionCalibrationSave|SetData _returnvalue_2 (.OutBodyCalibration (Class|CaptureDevice|GetCurrentCalibration (Variables|Default|GetCaptureDevice))))
  (SaveGame|SaveGametoSlot _returnvalue_2 (Variables|Default|GetEditorCalibrationFile)))

(event Custom|SetRecordingEnabled
  (params (IsEnabled :type Boolean))
  ;[0.3073 0.003134 0.009247] Toggle Animation Record
  (if IsEnabled
    (Utilities|TryRelocatetoCentre
      (:Out
        (bind _output_get (Variables|CaptureState|SetCaptureFile (Utilities|String|Append (Variables|Settings|GetSaveFolder) (Utilities|GenerateFileName))))
        (Development|ExecuteConsoleCommand (Utilities|String|Append "RecordAnimation " (Utilities|GetObjectName self) " " _output_get) 0)
        (CallFunction|UpdateStatus (Utilities|Text|ToText(String) (Utilities|String|Append "Capture started to: " (Variables|CaptureState|GetCaptureFile))) 0.0)
        (Variables|/Script/ViveMocapKit.CaptureDevice|SetbShowRefPose (Variables|Default|GetCaptureDevice) true)
        (Variables|CaptureState|SetIsRecording true)
        (Utilities|FlowControl|Delay 0.5)
        (Variables|/Script/ViveMocapKit.CaptureDevice|SetbShowRefPose (Variables|Default|GetCaptureDevice) false)))
    (else
      (Variables|CaptureState|SetIsRecording false)
      (Development|ExecuteConsoleCommand "StopRecordingAnimation all" (Game|GetPlayerController 0))
      (CallFunction|UpdateStatus (Utilities|Text|ToText(String) (Utilities|String|Append "Animation Sequence created:  " (Variables|CaptureState|GetCaptureFile))) 1e+01))))

(event Custom|FinishManualCalibration
  (bind _manualcalibrator (Variables|References|GetManualCalibrator))
  ;[1 1 1] Manual Calibration
  (Utilities|IsValid _manualcalibrator
    (:Is%20Valid
      (Default|DestroyMe _manualcalibrator))))

(event Custom|LoadCalibrationPresetAtTPose
  ;[1 1 1] Save/Load calibration
  (bind _returnvalue (SaveGame|LoadGamefromSlot (Variables|Default|GetCalibrationFile)))
  (bind _asbp_calibraton_file (Utilities|Casting|CastToBP_CalibratonFile _returnvalue))
  (bind _returnvalue_2 (Class|CaptureDevice|LoadCalibratedDatainTPoseEx (Variables|Default|GetCaptureDevice) (Variables|/Game/VMK/Blueprints/BP_CalibratonFile.BP_CalibratonFile_C|GetNewData _asbp_calibraton_file)))
  (if _returnvalue_2
    (Rendering|SetVisibility (Variables|Default|GetBodyMesh) true false)
    (Variables|CaptureState|SetState "NewEnumerator0")
    (Variables|CaptureState|SetIsCalibrated true)
    (Utilities|FlowControl|Delay 0.2)
    (Class|CaptureDevice|ToggleCapture (Variables|Default|GetCaptureDevice) true false)
    (Utilities|IsValid (Variables|References|GetMainMenuWidget)
      (:Is%20Valid
        (Default|OnPlayerCalibratied (Variables|References|GetMainMenuWidget))))))

(event Custom|OnMotionDevicesCalibration
  (params (NewCount :type Integer))
  (bind _wmenu_new_4 (Variables|Default|GetWMenu_New_4))
  ;[1 1 1] Update number of bones in collders
  (Utilities|IsValid _wmenu_new_4
    (:Is%20Valid
      (Default|UpdateStatus _wmenu_new_4 NewCount))))

(event Custom|StartManualCalibration
  ;[1 1 1] Manual Calibration
  (bind _returnvalue (Game|SpawnActorfromClass (Variables|Settings|GetManualCalibratorClass) (Math|Transform|MakeTransform "100.000000, 0, 0" "0,90.000000, 0") "Undefined" 0 (Variables|Default|GetCaptureDevice) 0))
  (Variables|References|SetManualCalibrator _returnvalue))

(event EventBeginPlay
  (bind _capturedevice (Variables|Default|GetCaptureDevice))
  ;[1 1 1] Initialize Capture Device and show Start Menu
  (Utilities|FlowControl|Delay 3.0)
  (|InitializeInputFromDevicesController)
  (|InitTrackerActors)
  (Class|CaptureDevice|LoadSkeletonSetupfromStruct _capturedevice (Variables|Settings|GetSkeletonPreset) true)
  (CallFunction|ShowMainMenu)
  (CallFunction|Menu1SelectBones)
  (CallFunction|UpdateStatus (Utilities|Text|FormatText "Application started with {num} Vive Trackers and Motion Controllers (minimum required: 4)" (Class|CaptureDevice|GetTrackingDevicesNum _capturedevice)) 0.0)
  (Class|CaptureDevice|InitializeFingers (Variables|Default|GetCaptureDevice) false))

(event Custom|UpdateStatus
  (params (Message :type Text) (Duration :type Float%20%28single-precision%29))
  (bind _mainmenuwidget (Variables|References|GetMainMenuWidget))
  ;[1 1 1] Update Status Bar
  (Utilities|IsValid _mainmenuwidget
    (:Is%20Valid
      (Default|SetStatus _mainmenuwidget Message)
      (if (> Duration 0.0)
        (Utilities|FlowControl|Delay Duration)
        (Default|SetStatus (Variables|References|GetMainMenuWidget))))))

(event Custom|Menu2_LoadCalibration
  (bind _returnvalue (UserInterface|CreateWidget "/Game/VMK/Slate/W_Wizard2DNew_02a_LoadCalib.W_Wizard2DNew_02a_LoadCalib_C" 0 5 "Take \"T\" pose and wait until timer expires"))
  (bind _output_get (Variables|Default|SetWMenu_New_2a _returnvalue))
  (UserInterface|Viewport|AddtoViewport _output_get 0)
  (Input|SetInputModeGameandUI (Game|GetPlayerController 0) _output_get "DoNotLock" false))

(event Custom|Menu_3_TPose
  (bind _returnvalue (UserInterface|CreateWidget "/Game/VMK/Slate/W_Wizard2DNew_02_PoseCalib.W_Wizard2DNew_02_PoseCalib_C" 0 5 "Take \"T\" pose and wait until timer expires"))
  (bind _output_get (Variables|Default|SetWMenu_New_3 _returnvalue))
  (UserInterface|Viewport|AddtoViewport _output_get 0)
  (Input|SetInputModeGameandUI (Game|GetPlayerController 0) _output_get "DoNotLock" false))

(event Custom|Menu_4_Calibration
  (bind _returnvalue (Game|Player|GetPlayerPawn 0))
  (bind (_loc _rot) (|GetBackPosition))
  (bind _returnvalue_2 (UserInterface|CreateWidget "/Game/VMK/Slate/W_Wizard2DNew_04_FullCalib.W_Wizard2DNew_04_FullCalib_C"))
  (bind _output_get (Variables|Default|SetWMenu_New_4 _returnvalue_2))
  (UserInterface|Viewport|AddtoViewport _output_get 0)
  (Input|SetInputModeGameandUI (Game|GetPlayerController 0) _output_get "DoNotLock" false)
  (Transformation|SetActorLocationAndRotation _returnvalue _loc _rot)
  (Pawn|SetControlRotation (Pawn|GetController _returnvalue) _rot))

(event Custom|SetModifyToolEnabled
  (params (IsEnabled :type Boolean))
  ;[1 1 1] Enable/Disable tool
  (bind _output_get (Variables|UI|SetHasModifyTool IsEnabled))
  (if _output_get
    (CallFunction|SpawnModifyTool "NewEnumerator0")
    (else
      (CallFunction|DestroyModifyTool))))

(event Custom|SpawnModifyTool
  (params (Type :type EModifyTool%20Enum :default "NewEnumerator0"))
  ;[1 1 1] Spawn New Modify Tool
  (CallFunction|DestroyModifyTool)
  (bind _output_get (Variables|UI|SetActiveTool Type))
  (bind _returnvalue (Game|SpawnActorfromClass (Utilities|Select :Index _output_get :NewEnumerator0 "/Game/VMK/Blueprints/Manipulators/BP_ToolTranslation.BP_ToolTranslation_C" :NewEnumerator1 "/Game/VMK/Blueprints/Manipulators/BP_ToolRotation.BP_ToolRotation_C" :NewEnumerator2 "/Game/VMK/Blueprints/Manipulators/BP_ToolScale.BP_ToolScale_C") (Math|Transform|MakeTransform "0, 0, 0") "AlwaysSpawn" 0 0))
  (bind _output_get_2 (Variables|UI|SetCurrentManipulator _returnvalue))
  (Transformation|AttachComponentToComponent _output_get_2 (Variables|Default|GetBodyMesh) "None" "SnapToTarget" "SnapToTarget" "KeepWorld" true)
  ;[1 1 1] Block Movement along Z Axis and rotation around roll/pitch axes, scale at Y axis
  (switch Utilities|FlowControl|Switch|SwitchonEModifyTool (Variables|UI|GetActiveTool)
    (:NewEnumerator0
      (bind _asbp_tool_translation (Utilities|Casting|CastToBP_ToolTranslation (Variables|UI|GetCurrentManipulator)))
      (Variables|/Game/VMK/Blueprints/Manipulators/BP_ToolTranslation.BP_ToolTranslation_C|SetActionFilter _asbp_tool_translation "1.000000,1.000000,0.000000"))
    (:NewEnumerator1
      (bind _asbp_tool_rotation (Utilities|Casting|CastToBP_ToolRotation (Variables|UI|GetCurrentManipulator)))
      (Variables|/Game/VMK/Blueprints/Manipulators/BP_ToolRotation.BP_ToolRotation_C|SetRotationFilter _asbp_tool_rotation "0,1.000000, 0"))
    (:NewEnumerator2
      (bind _asbp_tool_scale (Utilities|Casting|CastToBP_ToolScale (Variables|UI|GetCurrentManipulator)))
      (Variables|/Game/VMK/Blueprints/Manipulators/BP_ToolTranslation.BP_ToolTranslation_C|SetActionFilter _asbp_tool_scale "1.000000, 0,1.000000"))))

(event Custom|Menu2_ManualCalibration
  (bind _returnvalue (UserInterface|CreateWidget "/Game/VMK/Slate/W_Wizard2DNew_03_ManualCalib.W_Wizard2DNew_03_ManualCalib_C"))
  (bind _output_get (Variables|Default|SetWMenu_New_3a _returnvalue))
  (UserInterface|Viewport|AddtoViewport _output_get 0)
  (Input|SetInputModeGameandUI (Game|GetPlayerController 0) _output_get "DoNotLock" false))

(event Custom|DestroyModifyTool
  ;[1 1 1] Destroy current tool
  (Utilities|IsValid (Variables|UI|GetCurrentManipulator)
    (:Is%20Valid
      (Actor|DestroyActor (Variables|UI|GetCurrentManipulator)))))

(event Custom|ShowMenu_02_Setup
  ;[1 1 1] Show Menu Widgets
  (Widget|RemovefromParent (Variables|References|GetW_01_Scale))
  (bind _returnvalue (UserInterface|CreateWidget "/Game/VMK/Slate/W_Wizard2D_02_Settings.W_Wizard2D_02_Settings_C"))
  (bind _output_get (Variables|References|SetW_02_Settings _returnvalue))
  (UserInterface|Viewport|AddtoViewport _output_get 0))

(event Custom|ToggleModifyTool
  ;[1 1 1] Change current Modify tool
  (if (Variables|UI|GetHasModifyTool)
    (switch Utilities|FlowControl|Switch|SwitchonEModifyTool (Variables|UI|GetActiveTool)
      (:NewEnumerator0
        (CallFunction|SpawnModifyTool "NewEnumerator1"))
      (:NewEnumerator1
        (CallFunction|SpawnModifyTool "NewEnumerator2"))
      (:NewEnumerator2
        (CallFunction|SpawnModifyTool "NewEnumerator0")))))

(event Custom|ShowMainMenu
  ;[1 1 1] Show Menu Widgets
  (bind _returnvalue (UserInterface|CreateWidget "/Game/VMK/Slate/W_2D_MainMenu.W_2D_MainMenu_C"))
  (bind _output_get (Variables|References|SetMainMenuWidget _returnvalue))
  (UserInterface|Viewport|AddtoViewport _output_get 0))

(event Custom|ShowMenu_01_Scale
  (bind _returnvalue (Game|GetPlayerController 0))
  ;[1 1 1] Show Menu Widgets
  (bind _returnvalue_2 (UserInterface|CreateWidget "/Game/VMK/Slate/W_Wizard2D_01_Scale.W_Wizard2D_01_Scale_C"))
  (bind _output_get (Variables|References|SetW_01_Scale _returnvalue_2))
  (UserInterface|Viewport|AddtoViewport _output_get 0)
  (Input|SetInputModeUIOnly _returnvalue (Variables|References|GetW_01_Scale) "DoNotLock")
  (Variables|/Script/Engine.PlayerController|SetbShowMouseCursor _returnvalue true))

(event Custom|ShowCaptureMenu
  ;[1 1 1] Show Capture Menu
  (Utilities|IsValid (Variables|References|GetMainMenuWidget)
    (:Is%20Valid
      (Default|ShowCaptureMenu (Variables|References|GetMainMenuWidget)))))

(event Custom|ShowMenu_03_AutoCalibrate
  ;[1 1 1] Show Menu Widgets
  (Widget|RemovefromParent (Variables|References|GetW_02_Settings))
  (bind _returnvalue (UserInterface|CreateWidget "/Game/VMK/Slate/W_Wizard2D_03_Calibration.W_Wizard2D_03_Calibration_C"))
  (bind _output_get (Variables|References|SetW_03_AutoCalibration _returnvalue))
  (UserInterface|Viewport|AddtoViewport _output_get 0)
  (Input|SetInputModeGameandUI (Game|GetPlayerController 0) _output_get "DoNotLock" false))

(event Custom|Menu_1_SelectBones
  (bind _returnvalue (Game|GetPlayerController 0))
  (bind _returnvalue_2 (UserInterface|CreateWidget "/Game/VMK/Slate/W_Wizard2DNew_01_Bones.W_Wizard2DNew_01_Bones_C"))
  (bind _output_get (Variables|Default|SetWMenu_New_1 _returnvalue_2))
  (UserInterface|Viewport|AddtoViewport _output_get 0)
  (Input|SetInputModeUIOnly _returnvalue _output_get "DoNotLock")
  (Variables|/Script/Engine.PlayerController|SetbShowMouseCursor _returnvalue true))

(event Custom|Menu_2_ForwardDirection
  (bind _returnvalue (UserInterface|CreateWidget "/Game/VMK/Slate/W_Wizard2DNew_02_PoseCalib.W_Wizard2DNew_02_PoseCalib_C" 0 10 "Stand up and hold your hands forward" true))
  (bind _output_get (Variables|Default|SetWMenu_New_2 _returnvalue))
  (UserInterface|Viewport|AddtoViewport _output_get 0)
  (Input|SetInputModeGameandUI (Game|GetPlayerController 0) _output_get "DoNotLock" false))

(fn ConstructionScript)

(fn HasValidCalibrationFile
  (bind _returnvalue (SaveGame|LoadGamefromSlot (Variables|Default|GetCalibrationFile)))
  (Utilities|IsValid _returnvalue
    (:Is%20Valid
      (Utilities|Casting|CastToBP_CalibratonFile _returnvalue
        (:then
          (return true))
        (:CastFailed
          _)))
    (:Is%20Not%20Valid
      _))
  (return false))

(fn GetVisualTrackedDevices
  (return (Variables|Default|GetTrackingDevices)))