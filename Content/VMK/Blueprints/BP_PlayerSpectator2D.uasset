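; BP_PlayerSpectator2D is the player-side spectator that provides input controls for motion capture and manual tracker calibration.
; On BeginPlay it caches the first BP_CapturePawn2D and disables on-screen messages.
; SetActiveTracker stops control of the previous tracker and stores the new one, whose manipulation mode and space are toggled by input.
; Other inputs toggle body mesh and tracker visibility or recenter the pawn while capturing.
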(event Custom|SetActiveTracker
  (params (Actor :type BP%20Tracker%20Object%20Reference))
  ;[1 1 1] Update a pointer to currently selected tracker
  (Utilities|IsValid (Variables|Default|GetActiveTracker)
    (:Is%20Valid
      (Default|StopControl (Variables|Default|GetActiveTracker)))
    (:Is%20Not%20Valid
      _))
  (Variables|Default|SetActiveTracker Actor))

(event EventBeginPlay
  ;[1 1 1] Initialize Reference
  (bind _outactors (Actor|GetAllActorsOfClass "/Game/VMK/Blueprints/BP_CapturePawn2D.BP_CapturePawn2D_C"))
  (if (Utilities|Array|IsValidIndex _outactors)
    (Variables|Default|SetCapturePawn (Utilities|Array|Get(acopy) _outactors))
    (Development|ExecuteConsoleCommand "DisableAllScreenMessages" (Game|GetPlayerController 0))))

(event Input|ActionEvents|InputActionSwitchManipulator
  (params (Key :type Key%20Structure :default "None"))
  (bind _activetracker (Variables|Default|GetActiveTracker))
  ;[1 1 1] Manual Calibration Controls
  (:Pressed
    (Utilities|IsValid _activetracker
      (:Is%20Valid
        (if (Variables|/Game/VMK/Blueprints/BP_Tracker.BP_Tracker_C|GetKeyboardSelected _activetracker)
          (bind _output_get (Variables|Default|SetTrackerManipulateMode (not (Variables|Default|GetTrackerManipulateMode))))
          (Default|ToggleManipulationMode (Variables|Default|GetActiveTracker) _output_get))))))

(event Input|ActionEvents|InputActionToggleCapture
  (params (Key :type Key%20Structure :default "None"))
  (bind _capturepawn (Variables|Default|GetCapturePawn))
  ;[1 1 1] Manual Calibration Controls
  (:Pressed
    (Utilities|IsValid _capturepawn
      (:Is%20Valid
        (Rendering|ToggleVisibility (Variables|/Game/VMK/Blueprints/BP_CapturePawn2D.BP_CapturePawn2D_C|GetBodyMesh _capturepawn) false)))))

(event Input|ActionEvents|InputActionSwichManualCalibrationSpace
  (params (Key :type Key%20Structure :default "None"))
  (bind _activetracker (Variables|Default|GetActiveTracker))
  (:Pressed
    (Utilities|IsValid _activetracker
      (:Is%20Valid
        (Default|ToggleManipulatorSpace _activetracker)))))

(event Input|ActionEvents|InputActionShowHideMeshes
  (params (Key :type Key%20Structure :default "None"))
  ;[1 1 1] Helpers
  (:Pressed
    (bind _isa (Utilities|FlowControl|FlipFlop)
      (:A
        _)
      (:B
        _))
    (Default|SetTrackersVisibility (Variables|Default|GetCapturePawn) (not _isa))))

(event Input|ActionEvents|InputActionRelocateToCenter
  (params (Key :type Key%20Structure :default "None"))
  (bind _capturepawn (Variables|Default|GetCapturePawn))
  ;[1 1 1] Helpers
  (:Pressed
    (if (Class|CaptureDevice|IsCapturing (Variables|/Game/VMK/Blueprints/BP_CapturePawn2D.BP_CapturePawn2D_C|GetCaptureDevice _capturepawn))
      (Default|RelocatetoCenter _capturepawn))))

(fn ConstructionScript)