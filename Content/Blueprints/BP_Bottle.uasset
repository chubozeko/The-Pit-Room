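; BP_Bottle is a bottle actor that sets its mesh materials from its BottleType (Orange, Blue or White) and a floatable flag.
; UpdateBottleMaterials picks the Float or regular material set, varying the middle slot by type and sharing black and white plastics on the others.
; BeginPlay applies the regular set; nothing in this graph switches to the Float set.
; The regular White variant uses a green bottle material.
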(event EventBeginPlay
  (CallFunction|UpdateBottleMaterials false))

(fn ConstructionScript)

(fn UpdateBottleMaterials
  (params (IsFloatable :type Boolean))
  (bind _staticmeshcomponent (Variables|Debug|GetStaticMeshComponent))
  (bind _staticmeshcomponent_2 (Variables|Debug|GetStaticMeshComponent))
  (bind _staticmeshcomponent_3 (Variables|Debug|GetStaticMeshComponent))
  (bind _staticmeshcomponent_4 (Variables|Debug|GetStaticMeshComponent))
  (bind _staticmeshcomponent_5 (Variables|Debug|GetStaticMeshComponent))
  (bind _staticmeshcomponent_6 (Variables|Debug|GetStaticMeshComponent))
  (if IsFloatable
    (switch Utilities|FlowControl|Switch|SwitchonBottleType (Variables|Default|GetBottle%20Type)
      (:NewEnumerator0
        (Rendering|Material|SetMaterial _staticmeshcomponent_5 0 "/Game/Materials/Floatable/MI_Float_BlackPlastic.MI_Float_BlackPlastic")
        (Rendering|Material|SetMaterial _staticmeshcomponent_5 1 "/Game/Materials/Floatable/MI_Float_BottleOrange.MI_Float_BottleOrange")
        (Rendering|Material|SetMaterial _staticmeshcomponent_5 2 "/Game/Materials/Floatable/MI_Float_WhitePlastic.MI_Float_WhitePlastic"))
      (:NewEnumerator1
        (Rendering|Material|SetMaterial _staticmeshcomponent_3 0 "/Game/Materials/Floatable/MI_Float_BlackPlastic.MI_Float_BlackPlastic")
        (Rendering|Material|SetMaterial _staticmeshcomponent_3 1 "/Game/Materials/Floatable/MI_Float_BottleBlue.MI_Float_BottleBlue")
        (Rendering|Material|SetMaterial _staticmeshcomponent_3 2 "/Game/Materials/Floatable/MI_Float_WhitePlastic.MI_Float_WhitePlastic"))
      (:NewEnumerator2
        (Rendering|Material|SetMaterial _staticmeshcomponent_6 0 "/Game/Materials/Floatable/MI_Float_BlackPlastic.MI_Float_BlackPlastic")
        (Rendering|Material|SetMaterial _staticmeshcomponent_6 1 "/Game/Materials/Floatable/MI_Float_BottleWhite.MI_Float_BottleWhite")
        (Rendering|Material|SetMaterial _staticmeshcomponent_6 2 "/Game/Materials/Floatable/MI_Float_WhitePlastic.MI_Float_WhitePlastic")))
    (else
      (switch Utilities|FlowControl|Switch|SwitchonBottleType (Variables|Default|GetBottle%20Type)
        (:NewEnumerator0
          (Rendering|Material|SetMaterial _staticmeshcomponent_4 0 "/Game/Assets/BigCompanyArchViz/Materials/MI_ColorShinyBlackPlastic.MI_ColorShinyBlackPlastic")
          (Rendering|Material|SetMaterial _staticmeshcomponent_4 1 "/Game/Assets/BigCompanyArchViz/Materials/MI_FridgeBottleAOrange.MI_FridgeBottleAOrange")
          (Rendering|Material|SetMaterial _staticmeshcomponent_4 2 "/Game/Assets/BigCompanyArchViz/Materials/MI_ColorShinyWhitePlastic.MI_ColorShinyWhitePlastic"))
        (:NewEnumerator1
          (Rendering|Material|SetMaterial _staticmeshcomponent_2 0 "/Game/Assets/BigCompanyArchViz/Materials/MI_ColorShinyBlackPlastic.MI_ColorShinyBlackPlastic")
          (Rendering|Material|SetMaterial _staticmeshcomponent_2 1 "/Game/Assets/BigCompanyArchViz/Materials/MI_GlassBlue.MI_GlassBlue")
          (Rendering|Material|SetMaterial _staticmeshcomponent_2 2 "/Game/Assets/BigCompanyArchViz/Materials/MI_ColorShinyWhitePlastic.MI_ColorShinyWhitePlastic"))
        (:NewEnumerator2
          (Rendering|Material|SetMaterial _staticmeshcomponent 0 "/Game/Assets/BigCompanyArchViz/Materials/MI_ColorShinyBlackPlastic.MI_ColorShinyBlackPlastic")
          (Rendering|Material|SetMaterial _staticmeshcomponent 1 "/Game/Assets/BigCompanyArchViz/Materials/MI_FridgeBottleAGreen.MI_FridgeBottleAGreen")
          (Rendering|Material|SetMaterial _staticmeshcomponent 2 "/Game/Assets/BigCompanyArchViz/Materials/MI_ColorShinyWhitePlastic.MI_ColorShinyWhitePlastic"))))))