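; BP_DroppedBottleDetector is a volume actor that tracks which expected bottles lie inside its box.
; On begin overlap, it adds a BP_Bottle to CurrentBottles only if that bottle appears in ExpectedBottles, and on end overlap it removes it.
; CurrentBottles is cleared at BeginPlay, and IsEmpty reports whether any tracked bottles remain in the volume.
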(event OnComponentBeginOverlap(Box)
  (params (OverlappedComponent :type Primitive%20Component%20Object%20Reference) (OtherActor :type Actor%20Object%20Reference) (OtherComp :type Primitive%20Component%20Object%20Reference) (OtherBodyIndex :type Integer) (bFromSweep :type Boolean) (SweepResult :type Hit%20Result%20Structure%20%28by%20ref%29))
  (bind _asbp_bottle (Utilities|Casting|CastToBP_Bottle OtherActor))
  (bind _array_element (Utilities|Array|ForEachLoopwithBreak (Variables|Default|GetExpected%20Bottles) :!label _label)
    (:LoopBody
      (if (== _array_element _asbp_bottle)
        (Utilities|Array|Add (Variables|Default|GetCurrent%20Bottles) _asbp_bottle)
        (goto _label Break)))))

(event OnComponentEndOverlap(Box)
  (params (OverlappedComponent :type Primitive%20Component%20Object%20Reference) (OtherActor :type Actor%20Object%20Reference) (OtherComp :type Primitive%20Component%20Object%20Reference) (OtherBodyIndex :type Integer))
  (bind _asbp_bottle (Utilities|Casting|CastToBP_Bottle OtherActor))
  (Utilities|Array|RemoveItem (Variables|Default|GetCurrent%20Bottles) _asbp_bottle))

(event EventBeginPlay
  (Utilities|Array|Clear (Variables|Default|GetCurrent%20Bottles)))

(fn ConstructionScript)

(fn IsEmpty
  (return (Utilities|Array|IsEmpty (Variables|Default|GetCurrent%20Bottles))))