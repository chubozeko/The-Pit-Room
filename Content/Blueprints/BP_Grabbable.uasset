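; BP_Grabbable is an actor with a static mesh and a grab component, serving as a grabbable object with sound feedback.
; On BeginPlay it copies its GrabbedSFX and DroppedSFX variables into the GrabComponent.
; When it begins overlapping any actor other than a BP_CapturePawn, it plays DroppedSFX at the mesh's world location.
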(event EventBeginPlay
  (bind _grabcomponent (Variables|Default|GetGrabComponent))
  (Variables|/Game/VRTemplate/Blueprints/GrabComponent.GrabComponent_C|SetGrabbed%20SFX _grabcomponent (Variables|Default|GetGrabbed%20SFX))
  (Variables|/Game/VRTemplate/Blueprints/GrabComponent.GrabComponent_C|SetDropped%20SFX _grabcomponent (Variables|Default|GetDropped%20SFX)))

(event Collision|EventActorBeginOverlap
  (params (OtherActor :type Actor%20Object%20Reference))
  (Utilities|Casting|CastToBP_CapturePawn OtherActor
    (:CastFailed
      (Audio|PlaySoundatLocation (Variables|Default|GetDropped%20SFX) (Transformation|GetWorldLocation (Variables|Debug|GetStaticMeshComponent)) "0, 0, 0" 1.0 1.0 0.0 0 0 0 0))))

(event EventTick
  (params (DeltaSeconds :type Float%20%28single-precision%29)))

(fn ConstructionScript)