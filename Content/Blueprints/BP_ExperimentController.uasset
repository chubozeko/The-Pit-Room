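; Runs a VR motion-capture experiment through avatar selection, calibration, bottle interactions and a pit room, driven by input actions.
; Each stage change teleports the player, trackers, mirror and instructions panel via MoveTo, with level sequences handling screen fades.
; The BreakPSI pit room variant also spawns invisible floors after a delay.
; Records stage timestamps and bucket bottle counts, saving them to a text file before quitting.
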(event Custom|End%20Experiment
  (Default|StopTimer (Variables|Timers|GetTimer%20[Pit%20Room]))
  (Utilities|FlowControl|Delay 5.0)
  (CallFunction|FadetoBlack)
  (Variables|Logging|SetExperiment%20End%20Time (Math|DateTime|Now))
  (CallFunction|SaveExperimentData)
  (Utilities|FlowControl|Delay 2.0)
  (Game|QuitGame (Game|GetPlayerController 0) "Quit" false))

(event Custom|PrepareCalibration
  (bind _mocap_setup_menu (Variables|Default|GetMocap%20Setup%20Menu))
  (Default|ShowSetupMenu _mocap_setup_menu)
  (Default|CalibrateButton (Variables|/Game/VMK/Blueprints/BP_SetupMenu.BP_SetupMenu_C|GetW%20Wizard%2002%20Setup _mocap_setup_menu))
  (Default|ShowAutoCalibrationMenu _mocap_setup_menu)
  (Default|AutoFillTrackerBindings (Variables|/Game/VMK/Blueprints/BP_SetupMenu.BP_SetupMenu_C|GetW%20Wizard%2003%20AutoCal _mocap_setup_menu) (Variables|Default|GetTracker%20Bone%20Sequence)))

(event Custom|ResetPositionOnFloor
  (bind _asbp_capture_pawn (Utilities|Casting|CastToBP_CapturePawn (Variables|Default|GetPlayer%20Pawn)))
  (Default|RepositionAvatar _asbp_capture_pawn (.z (.location (Variables|PlayerPositions|GetCalibration%20Position)))))

(event Custom|GoToCalibrationStage
  (CallFunction|FadetoBlack)
  (Utilities|FlowControl|Delay 1.0)
  (Variables|Default|SetCurrent%20Stage "NewEnumerator0")
  (CallFunction|Moveto (Variables|PlayerPositions|GetCalibration%20Position) (Variables|Mirror|GetMirror%20Calibration%20Position) (Variables|Instructions|GetInstructions%20Calibration%20Position))
  (CallFunction|PrepareCalibration)
  (Utilities|FlowControl|Delay 0.5)
  (for _array_element (Variables|Training|GetAvatar%20Selector%20TV)
    (Rendering|SetActorHiddenInGame _array_element true))
  (Variables|Logging|SetCalibration%20Start%20Time (Math|DateTime|Now))
  (CallFunction|FadeIntoScene))

(event Custom|GoToInteractions
  (CallFunction|FadetoBlack)
  (Audio|PlaySoundatLocation "/Game/Audio/SoundCues/SC_Success.SC_Success" (.location (Variables|PlayerPositions|GetInteraction%20Position)) "0, 0, 0" 1.0 1.0 0.0 0 0 0 0)
  (Utilities|FlowControl|Delay 1.0)
  (Variables|Default|SetCurrent%20Stage "NewEnumerator2")
  (CallFunction|Moveto (Variables|PlayerPositions|GetInteraction%20Position) (Variables|Mirror|GetMirror%20Hidden%20Position) (Variables|Instructions|GetInstructions%20Interaction%20Position))
  (Default|StartTimer (Variables|Timers|GetTimer%20[Interactions]))
  (Utilities|FlowControl|Delay 0.5)
  (Variables|Logging|SetInteractions%20Start%20Time (Math|DateTime|Now))
  (CallFunction|FadeIntoScene))

(event EventBeginPlay
  (CallFunction|InvisibleScene)
  (Variables|Default|SetPlayer%20Pawn (Game|Player|GetPlayerPawn 0))
  (Variables|Logging|SetExperiment%20Start%20Time (Math|DateTime|Now))
  (bind _returnvalue (Actor|GetActorOfClass "/Game/Blueprints/BP_AvatarSelection.BP_AvatarSelection_C"))
  (Variables|Training|SetAvatar%20Selector _returnvalue))

(event Input|ActionEvents|InputActionResetPositionOnFloor
  (params (Key :type Key%20Structure :default "None"))
  (:Pressed
    (bind _asbp_capture_pawn (Utilities|Casting|CastToBP_CapturePawn (Variables|Default|GetPlayer%20Pawn)))
    (Default|RepositionAvatar _asbp_capture_pawn (.z (.location (Variables|PlayerPositions|GetCalibration%20Position))))))

(event Input|ActionEvents|InputActionGoToNextStage
  (params (Key :type Key%20Structure :default "None"))
  (:Pressed
    (switch Utilities|FlowControl|Switch|SwitchonExperimentStage (Variables|Default|GetCurrent%20Stage)
      (:NewEnumerator1
        (Default|SelectAvatar (Variables|Training|GetAvatar%20Selector))
        (CallFunction|GotoCalibrationStage))
      (:NewEnumerator0
        (bind _asbp_capture_pawn (Utilities|Casting|CastToBP_CapturePawn (Variables|Default|GetPlayer%20Pawn)))
        (if (Variables|/Game/VMK/Blueprints/BP_CapturePawn.BP_CapturePawn_C|GetIsCalibrated _asbp_capture_pawn)
          (CallFunction|GotoInteractions)))
      (:NewEnumerator2
        (if (Default|IsEmpty (Variables|Training|GetTable%20Dropped%20Bottle%20Detector))
          (Utilities|FlowControl|Delay 3.0)
          (CallFunction|FadetoBlack))))))

(event Input|ActionEvents|InputActionBeginPitRoom_Normal
  (params (Key :type Key%20Structure :default "None"))
  ;[0 0.1868 0.4844 0.5 14] Scary Pit Room
  (:Pressed
    (CallFunction|InvisibleScene)
    (Utilities|FlowControl|Delay 1.0)
    (Variables|Default|SetCurrent%20Stage "NewEnumerator3")
    (CallFunction|Moveto (Variables|PlayerPositions|GetPit%20Room%20Position) (Variables|Mirror|GetMirror%20Hidden%20Position) (Variables|Instructions|GetInstructions%20Pit%20Room%20Position))
    (Default|StartTimer (Variables|Timers|GetTimer%20[Pit%20Room]))
    (Default|StopTimer (Variables|Timers|GetTimer%20[Interactions]))
    (Rendering|SetActorHiddenInGame (Variables|PitRoom|GetPit%20Room%20Scoreboard) false)
    (Utilities|FlowControl|Delay 2.0)
    (Variables|Logging|SetPit%20Room%20Start%20Time (Math|DateTime|Now))
    (CallFunction|FadeIntoScene)))

(event Input|ActionEvents|InputActionBeginPitRoom_BreakPSI
  (params (Key :type Key%20Structure :default "None"))
  ;[0 0.1868 0.4844 0.5 14] Non-Scary Pit Room
  (:Pressed
    (CallFunction|InvisibleScene)
    (Utilities|FlowControl|Delay 1.0)
    (Variables|Default|SetCurrent%20Stage "NewEnumerator3")
    (CallFunction|Moveto (Variables|PlayerPositions|GetPit%20Room%20Position) (Variables|Mirror|GetMirror%20Hidden%20Position) (Variables|Instructions|GetInstructions%20Pit%20Room%20Position))
    (Default|StartTimer (Variables|Timers|GetTimer%20[Pit%20Room]))
    (Default|StopTimer (Variables|Timers|GetTimer%20[Interactions]))
    (Rendering|SetActorHiddenInGame (Variables|PitRoom|GetPit%20Room%20Scoreboard) false)
    (Utilities|FlowControl|Delay 2.0)
    (Variables|Logging|SetPit%20Room%20Start%20Time (Math|DateTime|Now))
    (CallFunction|FadeIntoScene)
    ;;[0 0.02016 0.04688 0.5] Invisible Floor
    (Utilities|FlowControl|Delay (Variables|PitRoom|GetFloor%20Spawn%20Time))
    (Variables|Logging|SetInvisible%20Floor%20Time (Math|DateTime|Now))
    (bind _returnvalue (Game|SpawnActorfromClass "/Game/Blueprints/BP_InvisibleFloor.BP_InvisibleFloor_C" (Variables|PitRoom|GetInvisible%20Floor%20Transform) "AlwaysSpawn" 0 0))
    (Variables|PitRoom|SetInvisible%20Floor _returnvalue)
    (bind _returnvalue_2 (Game|SpawnActorfromClass "/Game/Blueprints/BP_InvisibleFloor.BP_InvisibleFloor_C" (Variables|PitRoom|Get2nd%20Invisible%20Floor%20Transform) "AlwaysSpawn" 0 0))
    (Variables|PitRoom|SetInvisible%20Floor _returnvalue_2)))

(event Input|ActionEvents|InputActionStartPitRoom1
  (params (Key :type Key%20Structure :default "None"))
  (:Pressed
    (Game|OpenLevel(byObjectReference) "/Game/VMK/Maps/PitRoom1.PitRoom1")))

(event Input|ActionEvents|InputActionStartPitRoom2
  (params (Key :type Key%20Structure :default "None"))
  (:Pressed
    (Game|OpenLevel(byObjectReference) "/Game/VMK/Maps/PitRoom2.PitRoom2")))

(event Input|ActionEvents|InputActionPrepareForCalibrationStage
  (params (Key :type Key%20Structure :default "None"))
  (bind _mocap_setup_menu (Variables|Default|GetMocap%20Setup%20Menu))
  (:Pressed
    (Default|ShowSetupMenu _mocap_setup_menu)
    (Default|CalibrateButton (Variables|/Game/VMK/Blueprints/BP_SetupMenu.BP_SetupMenu_C|GetW%20Wizard%2002%20Setup _mocap_setup_menu))
    (Default|ShowAutoCalibrationMenu _mocap_setup_menu)
    (Default|AutoFillTrackerBindings (Variables|/Game/VMK/Blueprints/BP_SetupMenu.BP_SetupMenu_C|GetW%20Wizard%2003%20AutoCal _mocap_setup_menu) (Variables|Default|GetTracker%20Bone%20Sequence))))

(event Input|ActionEvents|InputActionEndExperiment
  (params (Key :type Key%20Structure :default "None"))
  (:Pressed
    (Default|StopTimer (Variables|Timers|GetTimer%20[Pit%20Room]))
    (Utilities|FlowControl|Delay 5.0)
    (CallFunction|FadetoBlack)
    (Variables|Logging|SetExperiment%20End%20Time (Math|DateTime|Now))
    (CallFunction|SaveExperimentData)
    (Utilities|FlowControl|Delay 2.0)
    (Game|QuitGame (Game|GetPlayerController 0) "Quit" false)))

(event Input|ActionEvents|InputActionGoToAvatarSelection
  (params (Key :type Key%20Structure :default "None"))
  (:Pressed
    (Variables|Default|SetCurrent%20Stage "NewEnumerator1")
    (CallFunction|Moveto (Variables|PlayerPositions|GetSelect%20Avatar%20Position) (Variables|Mirror|GetMirror%20Select%20Avatar%20Position) (Variables|Instructions|GetInstructions%20Select%20Avatar%20Position))
    (Utilities|FlowControl|Delay 2.0)
    (for _array_element (Variables|Training|GetAvatar%20Selector%20TV)
      (Rendering|SetActorHiddenInGame _array_element false))
    (Variables|Logging|SetAvatar%20Selection%20Start%20Time (Math|DateTime|Now))
    (CallFunction|FadeIntoScene)))

(event Input|ActionEvents|InputActionGoToCalibration
  (params (Key :type Key%20Structure :default "None"))
  (:Pressed
    (CallFunction|FadetoBlack)
    (Utilities|FlowControl|Delay 1.0)
    (Variables|Default|SetCurrent%20Stage "NewEnumerator0")
    (CallFunction|Moveto (Variables|PlayerPositions|GetCalibration%20Position) (Variables|Mirror|GetMirror%20Calibration%20Position) (Variables|Instructions|GetInstructions%20Calibration%20Position))
    (CallFunction|PrepareCalibration)
    (Utilities|FlowControl|Delay 0.5)
    (for _array_element (Variables|Training|GetAvatar%20Selector%20TV)
      (Rendering|SetActorHiddenInGame _array_element true))
    (Variables|Logging|SetCalibration%20Start%20Time (Math|DateTime|Now))
    (CallFunction|FadeIntoScene)))

(event Input|ActionEvents|InputActionGoToInteractions
  (params (Key :type Key%20Structure :default "None"))
  (:Pressed
    (CallFunction|FadetoBlack)
    (Audio|PlaySoundatLocation "/Game/Audio/SoundCues/SC_Success.SC_Success" (.location (Variables|PlayerPositions|GetInteraction%20Position)) "0, 0, 0" 1.0 1.0 0.0 0 0 0 0)
    (Utilities|FlowControl|Delay 1.0)
    (Variables|Default|SetCurrent%20Stage "NewEnumerator2")
    (CallFunction|Moveto (Variables|PlayerPositions|GetInteraction%20Position) (Variables|Mirror|GetMirror%20Hidden%20Position) (Variables|Instructions|GetInstructions%20Interaction%20Position))
    (Default|StartTimer (Variables|Timers|GetTimer%20[Interactions]))
    (Utilities|FlowControl|Delay 0.5)
    (Variables|Logging|SetInteractions%20Start%20Time (Math|DateTime|Now))
    (CallFunction|FadeIntoScene)))

(fn ConstructionScript)

(fn Moveto
  (params (Player%20Position :type Transform) (Mirror%20Position :type Transform) (Instructions%20Position :type Transform))
  (bind _instructions_panel (Variables|Instructions|GetInstructions%20Panel))
  (bind _returnvalue (Actor|GetActorOfClass "/SteamVRTrackingLib/Blueprints/BP_EditorViveTrackersController.BP_EditorViveTrackersController_C"))
  (Transformation|SetActorLocationAndRotation _returnvalue (.location Player%20Position) (.rotation Player%20Position) false true)
  (Transformation|SetActorLocationAndRotation (Variables|Default|GetPlayer%20Pawn) (.location Player%20Position) (.rotation Player%20Position) false true)
  (Transformation|SetActorLocationAndRotation (Variables|Mirror|GetMirror) (.location Mirror%20Position) (.rotation Mirror%20Position))
  (Transformation|SetActorLocationAndRotation _instructions_panel (.location Instructions%20Position) (.rotation Instructions%20Position))
  (Transformation|SetActorScale3D _instructions_panel (.scale Instructions%20Position))
  (CallFunction|UpdateInstructions)
  (bind _asbp_capture_pawn (Utilities|Casting|CastToBP_CapturePawn (Variables|Default|GetPlayer%20Pawn)))
  (Default|RepositionAvatar _asbp_capture_pawn (.Z (Math|Vector|BreakVector (.location Player%20Position)))))

(fn UpdateInstructions
  (bind _instructions_text (Variables|Instructions|GetInstructions%20Text))
  (bind _textrender (Variables|/Script/Engine.TextRenderActor|GetTextRender _instructions_text))
  (switch Utilities|FlowControl|Switch|SwitchonExperimentStage (Variables|Default|GetCurrent%20Stage)
    (:NewEnumerator1
      (Rendering|Components|TextRender|SetText _textrender (Variables|Instructions|GetInstr%20Avatar%20Selection)))
    (:NewEnumerator0
      (Rendering|Components|TextRender|SetText _textrender (Variables|Instructions|GetInstr%20Calibration)))
    (:NewEnumerator2
      (Rendering|Components|TextRender|SetText _textrender (Variables|Instructions|GetInstr%20Interactions)))
    (:NewEnumerator3
      (Rendering|Components|TextRender|SetText _textrender (Variables|Instructions|GetInstr%20Pit%20Room)))))

(fn FadetoBlack
  (bind _returnvalue (Actor|GetActorOfClass "/Script/LevelSequence.LevelSequenceActor"))
  (Class|LevelSequenceActor|SetSequence _returnvalue "/Game/Sequences/FadeOut.FadeOut")
  (Sequencer|Player|Play (Variables|/Script/LevelSequence.LevelSequenceActor|GetSequencePlayer _returnvalue) :!class /Script/MovieScene.MovieSceneSequencePlayer))

(fn FadeIntoScene
  (bind _returnvalue (Actor|GetActorOfClass "/Script/LevelSequence.LevelSequenceActor"))
  (Class|LevelSequenceActor|SetSequence _returnvalue "/Game/Sequences/FadeIn.FadeIn")
  (Sequencer|Player|Play (Variables|/Script/LevelSequence.LevelSequenceActor|GetSequencePlayer _returnvalue) :!class /Script/MovieScene.MovieSceneSequencePlayer))

(fn VisibleScene
  (bind _returnvalue (Actor|GetActorOfClass "/Script/LevelSequence.LevelSequenceActor"))
  (Class|LevelSequenceActor|SetSequence _returnvalue "/Game/Sequences/VisibleScreen.VisibleScreen")
  (Sequencer|Player|Play (Variables|/Script/LevelSequence.LevelSequenceActor|GetSequencePlayer _returnvalue) :!class /Script/MovieScene.MovieSceneSequencePlayer))

(fn InvisibleScene
  (bind _returnvalue (Actor|GetActorOfClass "/Script/LevelSequence.LevelSequenceActor"))
  (Class|LevelSequenceActor|SetSequence _returnvalue "/Game/Sequences/InvisibleScreen.InvisibleScreen")
  (Sequencer|Player|Play (Variables|/Script/LevelSequence.LevelSequenceActor|GetSequencePlayer _returnvalue) :!class /Script/MovieScene.MovieSceneSequencePlayer))

(fn LoadTrackerBoneSequence
  (params (TBS%20String :type String))
  (switch string TBS%20String
    (:Default
      (Variables|Default|SetTracker%20Bone%20Sequence "NewEnumerator2" :!label _label))
    (:LFoot,%20RFoot,%20Pelvis
      (goto _label))
    (:LFoot,%20Pelvis,%20RFoot
      (Variables|Default|SetTracker%20Bone%20Sequence "NewEnumerator3"))
    (:Pelvis,%20LFoot,%20RFoot
      (Variables|Default|SetTracker%20Bone%20Sequence "NewEnumerator0"))
    (:Pelvis,%20RFoot,%20LFoot
      (Variables|Default|SetTracker%20Bone%20Sequence "NewEnumerator1"))
    (:RFoot,%20LFoot,%20Pelvis
      (Variables|Default|SetTracker%20Bone%20Sequence "NewEnumerator4"))
    (:RFoot,%20Pelvis,%20LFoot
      (Variables|Default|SetTracker%20Bone%20Sequence "NewEnumerator5"))))

(fn SaveExperimentData
  (bind _returnvalue (Math|DateTime|Now))
  (Variables|Logging|SetTotal%20Bucket%20Capacities (Variables|/Game/Blueprints/BP_PaintBucket.BP_PaintBucket_C|GetMax%20Bottle%20Amount (Utilities|Array|Get(acopy) (Variables|PitRoom|GetBuckets))))
  (for _array_element (Variables|PitRoom|GetBuckets)
    (switch Utilities|FlowControl|Switch|SwitchonBottleType (Variables|/Game/Blueprints/BP_PaintBucket.BP_PaintBucket_C|GetBottle%20Type _array_element)
      (:NewEnumerator0
        (Variables|Logging|SetOrange%20Bottles%20Total (Variables|/Game/Blueprints/BP_PaintBucket.BP_PaintBucket_C|GetNumber%20of%20Bottles _array_element)))
      (:NewEnumerator1
        (Variables|Logging|SetBlue%20Bottles%20Total (Variables|/Game/Blueprints/BP_PaintBucket.BP_PaintBucket_C|GetNumber%20of%20Bottles _array_element)))
      (:NewEnumerator2
        (Variables|Logging|SetWhite%20Bottles%20Total (Variables|/Game/Blueprints/BP_PaintBucket.BP_PaintBucket_C|GetNumber%20of%20Bottles _array_element)))))
  (Class|BPFLTextFileManager|SaveArrayText (Utilities|String|Append (Class|KismetSystemLibrary|GetProjectSavedDirectory) "\\Experiments\\") (Utilities|String|Append "PRE-" (Utilities|String|ToString(Integer) (.year _returnvalue)) (Parsing|ParseInttoString (.month _returnvalue)) (Parsing|ParseInttoString (.day _returnvalue)) "_" (Parsing|ParseInttoString (.hour _returnvalue)) (Parsing|ParseInttoString (.minute _returnvalue)) (Parsing|ParseInttoString (.second _returnvalue)) ".txt") (Utilities|Array|MakeArray "Experiment ID: <entered by researcher>" (Utilities|String|Append "Experiment Start Time: " (Parsing|ParseDateTimetoString (Variables|Logging|GetExperiment%20Start%20Time))) (Utilities|String|Append "Avatar Selection Start Time: " (Parsing|ParseDateTimetoString (Variables|Logging|GetAvatar%20Selection%20Start%20Time))) (Utilities|String|Append "Calibration Start Time: " (Parsing|ParseDateTimetoString (Variables|Logging|GetCalibration%20Start%20Time))) (Utilities|String|Append "Interactions Start Time: " (Parsing|ParseDateTimetoString (Variables|Logging|GetInteractions%20Start%20Time))) (Utilities|String|Append "Pit Room Start Time: " (Parsing|ParseDateTimetoString (Variables|Logging|GetPit%20Room%20Start%20Time))) (Utilities|String|Append "Invisible Floor Spawn Time: " (Parsing|ParseDateTimetoString (Variables|Logging|GetInvisible%20Floor%20Time))) (Utilities|String|Append "Experiment End Time: " (Parsing|ParseDateTimetoString (Variables|Logging|GetExperiment%20End%20Time))) (Utilities|String|Append "Total Bucket Capacity: " (Utilities|String|ToString(Integer) (Variables|Logging|GetTotal%20Bucket%20Capacities))) (Utilities|String|Append "Orange Bucket Total: " (Utilities|String|ToString(Integer) (Variables|Logging|GetOrange%20Bottles%20Total))) (Utilities|String|Append "White Bucket Total: " (Utilities|String|ToString(Integer) (Variables|Logging|GetWhite%20Bottles%20Total))) (Utilities|String|Append "Blue Bucket Total: " (Utilities|String|ToString(Integer) (Variables|Logging|GetBlue%20Bottles%20Total)))) true)
  (return))

(fn ParseInttoString
  (params (Int :type Integer))
  (bind _returnvalue (Utilities|String|ToString(Integer) Int))
  (if (< Int 10)
    (LocalVariables|SetNew%20Int (Utilities|String|Append "0" _returnvalue))
    (else
      (LocalVariables|SetNew%20Int _returnvalue)))
  (return (LocalVariables|GetNew%20Int)))

(fn ParseDateTimetoString
  (params (Date%20Time :type Date%20Time%20Structure))
  (bind (_year _month _day _hour _minute _second _millisecond) (Math|DateTime|BreakDateTime Date%20Time))
  (return (Utilities|String|Append (Parsing|ParseInttoString _day) "/" (Parsing|ParseInttoString _month) "/" (Utilities|String|ToString(Integer) _year) " " (Parsing|ParseInttoString _hour) ":" (Parsing|ParseInttoString _minute) ":" (Parsing|ParseInttoString _second) ":" (Parsing|ParseInttoString _millisecond))))