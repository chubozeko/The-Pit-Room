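; BP_PaintBucket is a bucket that counts overlapping bottles of its own BottleType.
; Collision overlap plays a drop sound, then CheckBottle increments the count on a type match and refreshes the optional count/max text.
; One special BottleType hides the Color component and only plays a move sound, skipping counting.
; CheckBottle also supports removal clamped at zero, though the overlap only adds, and the maximum is display-only here.
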(event OnComponentBeginOverlap(Collision)
  (params (OverlappedComponent :type Primitive%20Component%20Object%20Reference) (OtherActor :type Actor%20Object%20Reference) (OtherComp :type Primitive%20Component%20Object%20Reference) (OtherBodyIndex :type Integer) (bFromSweep :type Boolean) (SweepResult :type Hit%20Result%20Structure%20%28by%20ref%29))
  (if (Utilities|Enum|Equal(Enum) (Variables|Default|GetBottle%20Type) "NewEnumerator3")
    (Audio|PlaySoundatLocation (Variables|Default|GetBucket%20Move%20SFX) (Transformation|GetWorldLocation (Variables|Default|GetCollision)) "0, 0, 0" 1.0 1.0 0.0 0 0 0 0)
    (else
      (Audio|PlaySoundatLocation (Variables|Default|GetDrop%20in%20Bucket%20SFX) (Transformation|GetWorldLocation (Variables|Default|GetCollision)) "0, 0, 0" 1.0 1.0 0.0 0 0 0 0)
      (bind _asbp_bottle (Utilities|Casting|CastToBP_Bottle OtherActor))
      (CallFunction|CheckBottle _asbp_bottle true)
      (CallFunction|UpdateBucketText))))

(event EventBeginPlay
  (bind _color (Variables|Default|GetColor))
  (CallFunction|UpdateBucketText)
  (if (Utilities|Enum|Equal(Enum) (Variables|Default|GetBottle%20Type) "NewEnumerator3")
    (Rendering|SetVisibility _color false false)
    (Development|SetHiddeninGame _color true false)
    (else
      (Rendering|SetVisibility _color true false)
      (Development|SetHiddeninGame _color false false)
      (if (Variables|Default|GetHasText)
        (Rendering|SetVisibility (Variables|/Script/Engine.TextRenderActor|GetTextRender (Variables|Default|GetBottles%20Text)) true false)))))

(fn ConstructionScript)

(fn UpdateBucketText
  (if (Variables|Default|GetHasText)
    (Rendering|Components|TextRender|SetText (Variables|/Script/Engine.TextRenderActor|GetTextRender (Variables|Default|GetBottles%20Text)) (Utilities|Text|ToText(String) (Utilities|String|Append (Utilities|String|ToString(Integer) (Variables|Default|GetNumber%20of%20Bottles)) " / " (Utilities|String|ToString(Integer) (Variables|Default|GetMax%20Bottle%20Amount)))))))

(fn CheckBottle
  (params (Bottle :type BP%20Bottle%20Object%20Reference) (Is%20Added :type Boolean))
  (if (Utilities|Enum|Equal(Enum) (Variables|/Game/Blueprints/BP_Bottle.BP_Bottle_C|GetBottle%20Type Bottle) (Variables|Default|GetBottle%20Type))
    (if Is%20Added
      (bind _result (Math|Integer|IncrementInt (Variables|Default|GetNumber%20of%20Bottles))
        (:%20%20
          (Variables|Default|SetNumber%20of%20Bottles _result)))
      (else
        (bind _result_2 (Math|Integer|DecrementInt (Variables|Default|GetNumber%20of%20Bottles))
          (:%20%20
            (if (< _result_2 0)
              (Variables|Default|SetNumber%20of%20Bottles 0)
              (else
                (Variables|Default|SetNumber%20of%20Bottles _result_2)))))))))