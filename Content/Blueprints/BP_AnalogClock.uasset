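; Analog clock actor that shows the current system time with rotating hour, minute and second hands.
; BeginPlay offsets each hand's initial pitch from Now(), adding for hours but subtracting for minutes and seconds.
; Tick feeds chained Delays that step the second hand each second, then minute and hour hands after waits computed from Now(), all in negative pitch.
; Tick-sound nodes exist but are disconnected.
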(event EventBeginPlay
  (bind _returnvalue (Math|DateTime|Now))
  (bind _minute_initial_rotation (Variables|Default|GetMinute%20Initial%20Rotation))
  (bind _second_initial_rotation (Variables|Default|GetSecond%20Initial%20Rotation))
  (bind _hour_initial_rotation (Variables|Default|GetHour%20Initial%20Rotation))
  ;[0.1384 0.2795 0.1109] Hours
  (Transformation|SetRelativeRotation (Variables|Default|GetHour_Hand) (Math|Rotator|MakeRotator (.roll _hour_initial_rotation) (+ (.pitch _hour_initial_rotation) (* (Math|Integer|%(Integer) (.hour _returnvalue) 12) 30)) (.yaw _hour_initial_rotation)) false false)
  ;[0.1384 0.2795 0.1109] Minutes
  (Transformation|SetRelativeRotation (Variables|Default|GetMin_Hand) (Math|Rotator|MakeRotator (.roll _minute_initial_rotation) (- (.pitch _minute_initial_rotation) (* (.minute _returnvalue) 6)) (.yaw _minute_initial_rotation)) false false)
  ;[0.1384 0.2795 0.1109] Seconds
  (Transformation|SetRelativeRotation (Variables|Default|GetSec_Hand) (Math|Rotator|MakeRotator (.roll _second_initial_rotation) (- (.pitch _second_initial_rotation) (* (.second _returnvalue) 6)) (.yaw _second_initial_rotation)) false false))

(event EventTick
  (params (DeltaSeconds :type Float%20%28single-precision%29))
  (bind _returnvalue (Math|DateTime|Now))
  ;[0.1384 0.2795 0.1109] Seconds
  (Utilities|FlowControl|Delay 1.0)
  (Transformation|AddLocalRotation (Variables|Default|GetSec_Hand) (Math|Rotator|MakeRotator 0.0 -6.0 0.0) false false)
  ;[0.1384 0.2795 0.1109] Minutes
  (Utilities|FlowControl|Delay (- 6e+01 (Math|Conversions|ToFloat(Integer) (.second _returnvalue))))
  (Transformation|AddLocalRotation (Variables|Default|GetMin_Hand) (Math|Rotator|MakeRotator 0.0 -6.0 0.0) false false)
  ;[0.1384 0.2795 0.1109] Hours
  (Utilities|FlowControl|Delay (* (- 6e+01 (Math|Conversions|ToFloat(Integer) (.minute _returnvalue))) 6e+01))
  (Transformation|AddLocalRotation (Variables|Default|GetHour_Hand) (Math|Rotator|MakeRotator 0.0 -3e+01 0.0) false false))

(fn ConstructionScript)