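; BP_CountdownTimer is an in-world countdown clock that shows minutes and seconds on a text render and plays tick and finish sounds.
; StartTimer resets to the configured time and enables counting, which Tick paces to one-second steps through a Delay while also tracking elapsed seconds.
; StopTimer, called directly or at zero, halts counting and tells BP_ExperimentController to update its instructions.
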(event Custom|Start%20Timer
  (CallFunction|ResetTimer)
  (Variables|Default|SetPlay%20Timer true))

(event Custom|Stop%20Timer
  (Variables|Default|SetPlay%20Timer false)
  (bind _returnvalue (Actor|GetActorOfClass "/Game/Blueprints/BP_ExperimentController.BP_ExperimentController_C"))
  (Default|UpdateInstructions _returnvalue))

(event Custom|Reset%20Timer
  (Variables|Default|SetRemaining%20Minutes (Variables|Default|GetTime%20in%20Minutes))
  (Variables|Default|SetRemaining%20Seconds (Variables|Default|GetTime%20in%20Seconds))
  (Variables|Default|SetTime%20Taken%20in%20Seconds 0)
  (Rendering|Components|TextRender|SetText (Variables|Default|GetTimerText) (Utilities|Text|FormatText "{mm}:{ss}" (Utilities|Text|ToText(Integer) (Variables|Default|GetRemaining%20Minutes) false true 2 2) (Utilities|Text|ToText(Integer) (Variables|Default|GetRemaining%20Seconds) false true 2 2))))

(event EventBeginPlay
  (CallFunction|ResetTimer))

(event EventTick
  (params (DeltaSeconds :type Float%20%28single-precision%29))
  (bind _timertext (Variables|Default|GetTimerText))
  (if (Variables|Default|GetPlay%20Timer)
    (Utilities|FlowControl|Delay 1.0)
    (Math|Integer|IncrementInt (Variables|Default|GetTime%20Taken%20in%20Seconds)
      (:%20%20
        (bind _result (Math|Integer|DecrementInt (Variables|Default|GetRemaining%20Seconds))
          (:%20%20
            (switch int _result
              (:Default
                (Rendering|Components|TextRender|SetText (Variables|Default|GetTimerText) (Utilities|Text|FormatText "{mm}:{ss}" (Utilities|Text|ToText(Integer) (Variables|Default|GetRemaining%20Minutes) false true 2 2) (Utilities|Text|ToText(Integer) (Variables|Default|GetRemaining%20Seconds) false true 2 2)) :!label _label)
                (Audio|PlaySoundatLocation (Variables|Default|GetTimer%20Tick) (Transformation|GetWorldLocation (Variables|Default|GetDefaultSceneRoot)) "0, 0, 0" 0.5 2.0 0.0 0 0 0 0))
              (:-1
                (if (<= (Variables|Default|GetRemaining%20Minutes) 0)
                  (Audio|PlaySoundatLocation (Variables|Default|GetTimer%20Finished) (Transformation|GetWorldLocation (Variables|Default|GetDefaultSceneRoot)) "0, 0, 0" 0.5 1.0 0.0 0 0 0 0)
                  (CallFunction|StopTimer)
                  (else
                    (bind _result_2 (Math|Integer|DecrementInt (Variables|Default|GetRemaining%20Minutes))
                      (:%20%20
                        (Variables|Default|SetRemaining%20Minutes _result_2)
                        (Variables|Default|SetRemaining%20Seconds 59)
                        (goto _label)))))))))))
    (else
      (Rendering|Components|TextRender|SetTextRenderColor _timertext (Variables|/Script/Engine.TextRenderComponent|GetTextRenderColor _timertext)))))

(fn ConstructionScript)