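; Avatar selection carousel that lets the player browse and pick a character preset during one specific BP_ExperimentController stage.
; On BeginPlay the presets are attached along a LinearDial at fixed spacing.
; Previous/Next inputs slide the dial in Tick for a set delay, snap it to the grid, update arrows and apply the preset to BP_CapturePawn.
; SelectAvatar reapplies the current preset and updates every BP_CloneMesh.
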(event Custom|CustomEvent_1
  ;[1 1 1] Version 1.1.3
)

(event Custom|SelectAvatar
  (bind _returnvalue (Actor|GetActorOfClass "/Game/Blueprints/BP_ExperimentController.BP_ExperimentController_C"))
  (if (Utilities|Enum|Equal(Enum) (Variables|/Game/Blueprints/BP_ExperimentController.BP_ExperimentController_C|GetCurrent%20Stage _returnvalue) "NewEnumerator1")
    (Default|SetDefault (Utilities|Array|Get(acopy) (Variables|Default|GetCharacter%20Presets) (Variables|Default|GetCurrent%20Character%20Index)))
    (bind _asbp_capture_pawn (Utilities|Casting|CastToBP_CapturePawn (Game|Player|GetPlayerPawn 0)))
    (Default|UpdateSkeletonSettings _asbp_capture_pawn)
    (bind _outactors (Actor|GetAllActorsOfClass "/Game/VMK/Blueprints/BP_CloneMesh.BP_CloneMesh_C"))
    (for _array_element _outactors
      (Default|UpdateClones _array_element)
      (Audio|PlaySoundatLocation (Variables|Default|GetSelect%20Avatar%20SFX) (Transformation|GetWorldLocation (Variables|/Script/Engine.Actor|GetRootComponent (Variables|Default|GetScreen))) "0, 0, 0" 1.0 1.0 0.0 0 0 0 0)
      (Utilities|FlowControl|Delay 1.0))))

(event EventTick
  (params (DeltaSeconds :type Float%20%28single-precision%29))
  (bind _linear_dial (Variables|Default|GetLinear%20Dial))
  (bind _linear_dial_2 (Variables|Default|GetLinear%20Dial))
  (bind _relativelocation (Variables|/Script/Engine.SceneComponent|GetRelativeLocation _linear_dial_2))
  (bind _relativelocation_2 (Variables|/Script/Engine.SceneComponent|GetRelativeLocation _linear_dial))
  (Variables|Default|SetDelta%20Seconds DeltaSeconds)
  (Utilities|FlowControl|Sequence
    (:then_0
      (if (Variables|Default|GetMove%20to%20Next%20Avatar)
        (Transformation|SetRelativeLocation (Variables|Default|GetLinear%20Dial) (Math|Vector|MakeVector (- (.x _relativelocation_2) (* (Variables|Default|GetSlide%20Speed) (Variables|Default|GetDelta%20Seconds))) (.y _relativelocation_2) (.z _relativelocation_2)) false false)))
    (:then_1
      (if (Variables|Default|GetMove%20to%20Previous%20Avatar)
        (Transformation|SetRelativeLocation (Variables|Default|GetLinear%20Dial) (Math|Vector|MakeVector (+ (.x _relativelocation) (* (Variables|Default|GetSlide%20Speed) (Variables|Default|GetDelta%20Seconds))) (.y _relativelocation) (.z _relativelocation)) false false)))))

(event EventBeginPlay
  (bind _returnvalue (Actor|GetActorOfClass "/Script/LevelSequence.LevelSequenceActor"))
  (Variables|Default|SetLevelSequencer _returnvalue)
  (Variables|Default|SetCurrent%20Character%20Index 0)
  (CallFunction|LoadCharacterPresets)
  (CallFunction|UpdateArrows))

(event Input|ActionEvents|InputActionPreviousAvatar
  (params (Key :type Key%20Structure :default "None"))
  ;[1 1 1] Version 1.1.3
)

(event Input|ActionEvents|InputActionNextAvatar
  (params (Key :type Key%20Structure :default "None"))
  ;[1 1 1] Version 1.1.3
)

(event Input|ActionEvents|InputActionPreviousAvatar
  (params (Key :type Key%20Structure :default "None"))
  (bind _linear_dial (Variables|Default|GetLinear%20Dial))
  (bind _relativelocation (Variables|/Script/Engine.SceneComponent|GetRelativeLocation _linear_dial))
  (:Pressed
    (if (not (or (Variables|Default|GetMove%20to%20Previous%20Avatar) (Variables|Default|GetMove%20to%20Next%20Avatar)))
      (bind _returnvalue (Actor|GetActorOfClass "/Game/Blueprints/BP_ExperimentController.BP_ExperimentController_C"))
      (if (Utilities|Enum|Equal(Enum) (Variables|/Game/Blueprints/BP_ExperimentController.BP_ExperimentController_C|GetCurrent%20Stage _returnvalue) "NewEnumerator1")
        (Rendering|SetActorHiddenInGame (Variables|Default|GetScreen) false)
        (if (> (Variables|Default|GetCurrent%20Character%20Index) 0)
          (Variables|Default|SetCurrent%20Character%20Index (- (Variables|Default|GetCurrent%20Character%20Index) 1))
          (Variables|Default|SetMove%20to%20Previous%20Avatar true)
          (Audio|PlaySoundatLocation (Variables|Default|GetSwitch%20Avatar%20SFX) (Transformation|GetWorldLocation (Variables|/Script/Engine.Actor|GetRootComponent (Variables|Default|GetScreen))) "0, 0, 0" 1.0 1.0 0.0 0 0 0 0)
          (CallFunction|UpdateArrows)
          (Utilities|FlowControl|Delay (Variables|Default|GetSlide%20Delay))
          (Variables|Default|SetMove%20to%20Previous%20Avatar false)
          (Transformation|SetRelativeLocation (Variables|Default|GetLinear%20Dial) (Math|Vector|MakeVector (Math|Float|SnapToGrid(Float) (.x _relativelocation) 2e+02) (.y _relativelocation) (.z _relativelocation)) false false))
        (Default|SetDefault (Utilities|Array|Get(acopy) (Variables|Default|GetCharacter%20Presets) (Variables|Default|GetCurrent%20Character%20Index)))
        (bind _asbp_capture_pawn (Utilities|Casting|CastToBP_CapturePawn (Game|Player|GetPlayerPawn 0)))
        (Default|UpdateSkeletonSettings _asbp_capture_pawn)
        (else
          (Rendering|SetActorHiddenInGame (Variables|Default|GetScreen) true))))))

(event Input|ActionEvents|InputActionNextAvatar
  (params (Key :type Key%20Structure :default "None"))
  (bind _linear_dial (Variables|Default|GetLinear%20Dial))
  (bind _relativelocation (Variables|/Script/Engine.SceneComponent|GetRelativeLocation _linear_dial))
  (:Pressed
    (if (not (or (Variables|Default|GetMove%20to%20Previous%20Avatar) (Variables|Default|GetMove%20to%20Next%20Avatar)))
      (bind _returnvalue (Actor|GetActorOfClass "/Game/Blueprints/BP_ExperimentController.BP_ExperimentController_C"))
      (if (Utilities|Enum|Equal(Enum) (Variables|/Game/Blueprints/BP_ExperimentController.BP_ExperimentController_C|GetCurrent%20Stage _returnvalue) "NewEnumerator1")
        (Rendering|SetActorHiddenInGame (Variables|Default|GetScreen) false)
        (if (< (Variables|Default|GetCurrent%20Character%20Index) (Utilities|Array|LastIndex (Variables|Default|GetCharacter%20Presets)))
          (Variables|Default|SetCurrent%20Character%20Index (+ (Variables|Default|GetCurrent%20Character%20Index) 1))
          (Variables|Default|SetMove%20to%20Next%20Avatar true)
          (Audio|PlaySoundatLocation (Variables|Default|GetSwitch%20Avatar%20SFX) (Transformation|GetWorldLocation (Variables|/Script/Engine.Actor|GetRootComponent (Variables|Default|GetScreen))) "0, 0, 0" 1.0 1.0 0.0 0 0 0 0)
          (CallFunction|UpdateArrows)
          (Utilities|FlowControl|Delay (Variables|Default|GetSlide%20Delay))
          (Variables|Default|SetMove%20to%20Next%20Avatar false)
          (Transformation|SetRelativeLocation (Variables|Default|GetLinear%20Dial) (Math|Vector|MakeVector (Math|Float|SnapToGrid(Float) (.x _relativelocation) 2e+02) (.y _relativelocation) (.z _relativelocation)) false false))
        (Default|SetDefault (Utilities|Array|Get(acopy) (Variables|Default|GetCharacter%20Presets) (Variables|Default|GetCurrent%20Character%20Index)))
        (bind _asbp_capture_pawn (Utilities|Casting|CastToBP_CapturePawn (Game|Player|GetPlayerPawn 0)))
        (Default|UpdateSkeletonSettings _asbp_capture_pawn)
        (else
          (Rendering|SetActorHiddenInGame (Variables|Default|GetScreen) true))))))

(fn ConstructionScript)

(fn UpdateArrows
  (bind _current_character_index (Variables|Default|GetCurrent%20Character%20Index))
  ;[0.2471 0.287 0.4948 0.573] Version 2.0.0
  ;;[0.2031 0.2031 0.2031 0.663 16] Show/Hide Arrows
  (if (== _current_character_index 0)
    (Rendering|SetVisibility (Variables|/Script/Engine.Actor|GetRootComponent (Variables|Default|GetLeft%20Arrow)) false true)
    (Rendering|SetVisibility (Variables|/Script/Engine.Actor|GetRootComponent (Variables|Default|GetRight%20Arrow)) true true)
    (elif (== _current_character_index (Utilities|Array|LastIndex (Variables|Default|GetCharacter%20Presets)))
      (Rendering|SetVisibility (Variables|/Script/Engine.Actor|GetRootComponent (Variables|Default|GetLeft%20Arrow)) true true)
      (Rendering|SetVisibility (Variables|/Script/Engine.Actor|GetRootComponent (Variables|Default|GetRight%20Arrow)) false true)
      (else
        (Rendering|SetVisibility (Variables|/Script/Engine.Actor|GetRootComponent (Variables|Default|GetLeft%20Arrow)) true true)
        (Rendering|SetVisibility (Variables|/Script/Engine.Actor|GetRootComponent (Variables|Default|GetRight%20Arrow)) true true)))))

(fn UpdateSkeletalMeshandAnimation
  (params (Target%20Mesh :type Skeletal%20Mesh%20Component%20Object%20Reference) (Skeleton%20Preset :type BP%20Skeleton%20Preset%20Object%20Reference) (Is%20Visible :type Boolean))
  (if Is%20Visible
    (Class|SkinnedMeshComponent|SetSkeletalMesh Target%20Mesh (Variables|/Game/VMK/Blueprints/BP_SkeletonPreset.BP_SkeletonPreset_C|GetSkeletalMesh Skeleton%20Preset) false)
    (Components|Animation|SetAnimation Target%20Mesh (.animtoplay (Variables|/Script/Engine.SkeletalMeshComponent|GetAnimationData (Variables|/Game/VMK/Blueprints/BP_SkeletonPreset.BP_SkeletonPreset_C|GetAvatar Skeleton%20Preset))))
    (Rendering|SetVisibility Target%20Mesh Is%20Visible false)
    (else
      (Rendering|SetVisibility Target%20Mesh Is%20Visible false))))

(fn GetCharacterfromPresets
  (params (Index :type Integer))
  (return (Variables|/Game/VMK/Blueprints/BP_SkeletonPreset.BP_SkeletonPreset_C|GetAvatar (Utilities|Array|Get(acopy) (Variables|Default|GetCharacter%20Presets) Index))))

(fn LoadCharacterPresets
  (for (_array_element _array_index) (Variables|Default|GetCharacter%20Presets)
    (Transformation|AttachComponentToComponent _array_element (Variables|Default|GetLinear%20Dial) "None" "KeepRelative" "KeepRelative" "KeepRelative" true)
    (Transformation|SetActorRelativeLocation _array_element (Math|Vector|MakeVector (* _array_index 2e+02) 0.0 0.0) false true)))